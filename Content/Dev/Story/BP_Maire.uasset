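; Mayor NPC that guides the player through a tutorial tour, walking between goal actors after dialogs.
; After each dialog he AI-moves to the next goal, with a black-transition teleport as fallback if the move fails, then advances the line.
; During the tutorial, a looping timer detects a player straying too far, opens a call-back dialog, then teleports them back beside him once it ends.
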(event Custom|distance%20test
  (bind _as_bp_third_person_character (Variables|Default|GetAs%20BP%20Third%20Person%20Character))
  (if (Variables|/Game/ThirdPerson/Blueprints/BP_ThirdPersonGameMode.BP_ThirdPersonGameMode_C|GetIn_tutorial (Variables|Default|GetAs%20BP%20Third%20Person%20Game%20Mode))
    (if (>= (Transformation|GetDistanceTo self (Variables|Default|GetAs%20BP%20Third%20Person%20Character)) 6.5e+02)
      (Utilities|Time|ClearandInvalidateTimerbyHandle (Variables|Default|Gettimer))
      (Utilities|FlowControl|DoOnce false
        (:Completed
          (bind _returnvalue (UserInterface|CreateWidget "/Game/UI/Story/WB_Dialog_system.WB_Dialog_system_C" 0 (Utilities|Array|MakeArray (Variables|Default|GetChara_name)) (Utilities|Array|MakeArray "Attends ! J'ai pas fini de te faire visiter !") false self false true))
          (UserInterface|Viewport|AddtoViewport _returnvalue 0)
          (Transformation|SetWorldRotation (Variables|/Script/Engine.Character|GetCapsuleComponent _as_bp_third_person_character) (Math|Rotator|FindLookatRotation (Transformation|GetActorLocation _as_bp_third_person_character) (Transformation|GetActorLocation)) false false)
          (Variables|Default|SetTP%20? true))))))

(event Custom|quest_init
  (bind _returnvalue (Utilities|Time|SetTimerbyEvent (delegate Custom|distance%20test) 0.1 true))
  (Variables|Default|Settimer _returnvalue))

(event Custom|reset%20do%20once
  (bind _as_bp_third_person_character (Variables|Default|GetAs%20BP%20Third%20Person%20Character))
  (Utilities|FlowControl|DoOnce false) ; enters at Reset
)

(event EventBeginPlay
  (|CallParentFunction) ; This node is disabled and will not be called.\nDrag off pins to build functionality.
)

(event Collision|EventActorBeginOverlap
  (params (OtherActor :type Actor%20Object%20Reference))
  (|CallParentFunction OtherActor) ; This node is disabled and will not be called.\nDrag off pins to build functionality.
)

(event EventTick
  (params (DeltaSeconds :type Float%20%28single-precision%29))
  (|CallParentFunction DeltaSeconds) ; This node is disabled and will not be called.\nDrag off pins to build functionality.
)

(event EventPostDialogEvent
  (bind _returnvalue (Transformation|GetActorLocation))
  (bind _goals (Variables|Default|GetGoals))
  (bind _line (Variables|Default|Getline))
  (bind _as_bp_third_person_character (Variables|Default|GetAs%20BP%20Third%20Person%20Character))
  (bind _output (Utilities|Array|Get(acopy) _goals _line))
  (if (Variables|Default|Getactivate%20tuto%20?)
    (Variables|/Game/ThirdPerson/Blueprints/BP_ThirdPersonGameMode.BP_ThirdPersonGameMode_C|SetIn_tutorial (.AsBP%20Third%20Person%20Game%20Mode (Utilities|Casting|CastToBP_ThirdPersonGameMode (Game|GetGameMode))) true))
  (if (Variables|Default|GetTP%20?)
    (bind _returnvalue_2 (UserInterface|CreateWidget "/Game/UI/WB_Transi_Black.WB_Transi_Black_C"))
    (UserInterface|Viewport|AddtoViewport _returnvalue_2 0)
    (Utilities|FlowControl|Delay 1.2)
    (Transformation|SetWorldLocation (Variables|/Script/Engine.Character|GetCapsuleComponent (Variables|Default|GetAs%20BP%20Third%20Person%20Character)) (Math|Vector|MakeVector (+ (.x _returnvalue) -1.5e+02) (.y _returnvalue) (.z _returnvalue)) false false)
    (Variables|Default|SetTP%20? false)
    (CallFunction|QuestInit)
    (Transformation|SetWorldRotation (Variables|/Script/Engine.Character|GetCapsuleComponent _as_bp_third_person_character) (Math|Rotator|FindLookatRotation (Transformation|GetActorLocation _as_bp_third_person_character) (Transformation|GetActorLocation)) false false)
    (CallFunction|ResetDoOnce)
    (else
      (AI|AIMoveTo self "0, 0, 0" _output 5.0 false
        (:then
          (Variables|Default|SetCan_talk%20? false))
        (:OnSuccess
          (Transformation|SetWorldRotation (Variables|Default|GetCapsuleComponent) (Transformation|GetWorldRotation (Variables|/Game/Dev/BP_TP_Point.BP_TP_Point_C|GetDefaultSceneRoot _output)) false false :!label _label)
          (Actor|DestroyActor _output)
          (Math|Integer|IncrementInt (Variables|Default|Getline)
            (:%20%20
              (CallFunction|QuestInit)
              (Variables|Default|SetCan_talk%20? true))))
        (:OnFail
          (Utilities|IsValid _output
            (:Is%20Valid
              (bind _returnvalue_3 (UserInterface|CreateWidget "/Game/UI/WB_Transi_Black.WB_Transi_Black_C"))
              (UserInterface|Viewport|AddtoViewport _returnvalue_3 0)
              (Utilities|FlowControl|Delay 1.2)
              (Transformation|SetWorldLocation (Variables|Default|GetCapsuleComponent) (Transformation|GetActorLocation _output) false false)
              (Variables|/Game/ThirdPerson/Blueprints/BP_ThirdPersonGameMode.BP_ThirdPersonGameMode_C|SetIn_tutorial (Variables|Default|GetAs%20BP%20Third%20Person%20Game%20Mode) false)
              (goto _label))))))))

(fn ConstructionScript
  (|CallParentFunction))