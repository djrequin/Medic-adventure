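; Story trigger volume that starts a dialog during the tutorial sequence, acting only when the game mode's TutoIndex matches its SelfIndex.
; When the third-person character overlaps the box, it increments its own SelfIndex and shows a WB_Dialog_system widget.
; The widget receives speaker names converted from enums, the dialog contents, and the Maire NPC with its post-dialog event.
; The trigger then destroys itself, so it fires only once.
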(event OnComponentBeginOverlap(Box)
  (params (OverlappedComponent :type Primitive%20Component%20Object%20Reference) (OtherActor :type Actor%20Object%20Reference) (OtherComp :type Primitive%20Component%20Object%20Reference) (OtherBodyIndex :type Integer) (bFromSweep :type Boolean) (SweepResult :type Hit%20Result%20Structure%20%28by%20ref%29))
  (bind _maire (Variables|Default|GetMaire))
  (Utilities|Casting|CastToBP_ThirdPersonCharacter OtherActor)
  (if (== (Variables|/Game/ThirdPerson/Blueprints/BP_ThirdPersonGameMode.BP_ThirdPersonGameMode_C|GetTuto_index (.AsBP%20Third%20Person%20Game%20Mode (Utilities|Casting|CastToBP_ThirdPersonGameMode (Game|GetGameMode)))) (Variables|Default|GetSelf_index))
    (Math|Integer|IncrementInt (Variables|Default|GetSelf_index)
      (:%20%20
        (bind _returnvalue (UserInterface|CreateWidget "/Game/UI/Story/WB_Dialog_system.WB_Dialog_system_C" 0 (CallFunction|ConvertNames) (Variables|Default|GetContents) false _maire false (Variables|/Game/Dev/Story/BP_Chara_Parent.BP_Chara_Parent_C|GetPost_dialog_event? _maire)))
        (UserInterface|Viewport|AddtoViewport _returnvalue 0)
        (Actor|DestroyActor)))))

(event EventBeginPlay)

(event Collision|EventActorBeginOverlap
  (params (OtherActor :type Actor%20Object%20Reference)))

(event EventTick
  (params (DeltaSeconds :type Float%20%28single-precision%29)))

(fn ConstructionScript)

(fn ConvertNames
  (for _array_element (Variables|Default|GetNames)
    (Utilities|Array|Add (LocalVariables|GetNames) (Utilities|String|EnumtoString _array_element)))
  (return (LocalVariables|GetNames)))