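; BP_Max is a story NPC who asks the player to find a lost bracelet, with French dialogue.
; The upper choice searches the player's RandomObjects for an actor tagged BQ1, destroys it if found, then thanks the player, updates dialogue and quest state and sets CanBeSick.
; After the success dialogue, PostDialogEvent shows money and experience reward widgets.
; A missing bracelet gets a disappointed reply, while the bottom choice gets simple thanks.
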(event EventBeginPlay
  (|CallParentFunction) ; This node is disabled and will not be called.\nDrag off pins to build functionality.
)

(event Collision|EventActorBeginOverlap
  (params (OtherActor :type Actor%20Object%20Reference))
  (|CallParentFunction OtherActor) ; This node is disabled and will not be called.\nDrag off pins to build functionality.
)

(event EventTick
  (params (DeltaSeconds :type Float%20%28single-precision%29))
  (|CallParentFunction DeltaSeconds) ; This node is disabled and will not be called.\nDrag off pins to build functionality.
)

(event EventUpperChoice
  (params (Widget :type WB%20Dialog%20System%20Object%20Reference))
  (bind _chara_name (Variables|Default|GetChara_name))
  (bind _chara_name_2 (Variables|Default|GetChara_name))
  (Widget|RemovefromParent Widget)
  (bind _found__ (CallFunction|CheckBracelet))
  (if _found__
    (bind _returnvalue (UserInterface|CreateWidget "/Game/UI/Story/WB_Dialog_system.WB_Dialog_system_C" 0 (Utilities|Array|MakeArray _chara_name_2 _chara_name_2) (Utilities|Array|MakeArray "Oh tu l'as trouvé ! Merci infiniment pour ton aide !" "Tiens, pour te remercier. ") false self false true))
    (UserInterface|Viewport|AddtoViewport _returnvalue 0)
    (Utilities|FlowControl|Sequence
      (:then_0
        (Variables|Default|SetPost_dialog_choice? false)
        (Variables|Default|SetCanBeSick true))
      (:then_1
        (Variables|Default|SetContents (Utilities|Array|MakeArray "Merci encore d'avoir retrouvé mon bracelet, il a une valeur inestimable à mes yeux.")))
      (:then_2
        (Variables|Default|SetH_Names (Utilities|Array|MakeArray (Variables|Default|GetChara_name))))
      (:then_3
        (CallFunction|QuestInits false)))
    (else
      (bind _returnvalue_2 (UserInterface|CreateWidget "/Game/UI/Story/WB_Dialog_system.WB_Dialog_system_C" 0 (Utilities|Array|MakeArray _chara_name _chara_name) (Utilities|Array|MakeArray "Ah. Tu me dis ça, mais je vois bien que tu ne l'a pas en ta possession." "C'est pas très sympa de me faire espérer comme ça...") false self))
      (UserInterface|Viewport|AddtoViewport _returnvalue_2 0))))

(event EventBottomChoice
  (params (Widget :type WB%20Dialog%20System%20Object%20Reference))
  (Widget|RemovefromParent Widget)
  (bind _returnvalue (UserInterface|CreateWidget "/Game/UI/Story/WB_Dialog_system.WB_Dialog_system_C" 0 (Utilities|Array|MakeArray (Variables|Default|GetChara_name)) (Utilities|Array|MakeArray "Merci infiniment, je compte sur toi !") false self))
  (UserInterface|Viewport|AddtoViewport _returnvalue 0))

(event EventPostDialogEvent
  (bind _returnvalue (UserInterface|CreateWidget "/Game/UI/WB_Money_Changes.WB_Money_Changes_C" 0 true 15))
  (Default|OperateChange _returnvalue)
  (UserInterface|Viewport|AddtoViewport _returnvalue 0)
  (bind _returnvalue_2 (UserInterface|CreateWidget "/Game/UI/WB_Exp_receive.WB_Exp_receive_C" 0 15.0))
  (UserInterface|Viewport|AddtoViewport _returnvalue_2 0))

(fn ConstructionScript
  (|CallParentFunction))

(fn CheckBracelet
  (bind _array_element (Utilities|Array|ForEachLoopwithBreak (Variables|/Game/ThirdPerson/Blueprints/BP_ThirdPersonCharacter.BP_ThirdPersonCharacter_C|GetRandom_objects (Variables|Default|GetAs%20BP%20Third%20Person%20Character)) :!label _label)
    (:LoopBody
      (Utilities|IsValid _array_element
        (:Is%20Valid
          (if (Actor|ActorHasTag _array_element "BQ1")
            (LocalVariables|Setfound true)
            (Actor|DestroyActor _array_element)
            (goto _label Break)))))
    (:Completed
      (return (LocalVariables|Getfound)))))