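; Story NPC Blueprint for Lina, who offers the player a rank check or gameplay advice in French.
; Implements two choice events that each close the calling widget: the upper opens WB_Rank with Lina as PNJ, the lower opens WB_Dialog_system with hints on gathering ingredients, preparing medicine at the guild and helping villagers.
; PostDialogEvent shows a closing line inviting the player to return.
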(event EventBeginPlay
  (|CallParentFunction))

(event Collision|EventActorBeginOverlap
  (params (OtherActor :type Actor%20Object%20Reference))
  (|CallParentFunction OtherActor) ; This node is disabled and will not be called.\nDrag off pins to build functionality.
)

(event EventTick
  (params (DeltaSeconds :type Float%20%28single-precision%29))
  (|CallParentFunction DeltaSeconds) ; This node is disabled and will not be called.\nDrag off pins to build functionality.
)

(event EventUpperChoice
  (params (Widget :type WB%20Dialog%20System%20Object%20Reference))
  (Widget|RemovefromParent Widget)
  (bind _returnvalue (UserInterface|CreateWidget "/Game/UI/WB_Rank.WB_Rank_C" 0 self))
  (UserInterface|Viewport|AddtoViewport _returnvalue 0))

(event EventBottomChoice
  (params (Widget :type WB%20Dialog%20System%20Object%20Reference))
  (bind _chara_name (Variables|Default|GetChara_name))
  (Widget|RemovefromParent Widget)
  (bind _returnvalue (UserInterface|CreateWidget "/Game/UI/Story/WB_Dialog_system.WB_Dialog_system_C" 0 (Utilities|Array|MakeArray _chara_name _chara_name _chara_name) (Utilities|Array|MakeArray "Voyons voir... Est-ce que tu as exploré les plaines ? Tu pourrais y trouver de superbes ingrédients pour concoter tes médicaments." "Quand tu auras trouvé ton bonheur, rend toi dans la pièce en bas de la guilde pour préparer tes médicaments. Je suis désolée, mais la procédure veut que tu te trouves dans cette pièce pour en préparer." "Ou sinon tu peux aider les villageois en difficulté. Ce ne sont pas les occupations qui manquent !") false 0))
  (UserInterface|Viewport|AddtoViewport _returnvalue 0))

(event EventPostDialogEvent
  (bind _returnvalue (UserInterface|CreateWidget "/Game/UI/Story/WB_Dialog_system.WB_Dialog_system_C" 0 (Utilities|Array|MakeArray "Lina") (Utilities|Array|MakeArray "N'hésite pas à revenir  me voir pour consulter ton rang ou me demander des conseils !") false 0))
  (UserInterface|Viewport|AddtoViewport _returnvalue 0))

(fn ConstructionScript
  (|CallParentFunction))