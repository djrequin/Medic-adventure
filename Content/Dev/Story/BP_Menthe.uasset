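; Dialogue NPC Menthe, who tells the player, addressed as an apothecary, which villagers of Eudépar are sick.
; The upper choice runs GetContent, which scans the game mode's NPC list and packs sick names into French lines of up to three, plus a closing or nobody-sick line.
; Those lines and matching speaker names feed a new WB_Dialog_system widget.
; The bottom choice opens the same widget with a farewell.
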(event EventBeginPlay
  (|CallParentFunction) ; This node is disabled and will not be called.\nDrag off pins to build functionality.
)

(event Collision|EventActorBeginOverlap
  (params (OtherActor :type Actor%20Object%20Reference))
  (|CallParentFunction OtherActor) ; This node is disabled and will not be called.\nDrag off pins to build functionality.
)

(event EventTick
  (params (DeltaSeconds :type Float%20%28single-precision%29))
  (|CallParentFunction DeltaSeconds) ; This node is disabled and will not be called.\nDrag off pins to build functionality.
)

(event EventUpperChoice
  (params (Widget :type WB%20Dialog%20System%20Object%20Reference))
  (Widget|RemovefromParent Widget)
  (CallFunction|GetContent)
  (bind _returnvalue (UserInterface|CreateWidget "/Game/UI/Story/WB_Dialog_system.WB_Dialog_system_C" 0 (Variables|Default|GetNew_names) (Variables|Default|Getsick%20people) false self))
  (UserInterface|Viewport|AddtoViewport _returnvalue 0))

(event EventBottomChoice
  (params (Widget :type WB%20Dialog%20System%20Object%20Reference))
  (Widget|RemovefromParent Widget)
  (bind _returnvalue (UserInterface|CreateWidget "/Game/UI/Story/WB_Dialog_system.WB_Dialog_system_C" 0 (Utilities|Array|MakeArray (Variables|Default|GetChara_name)) (Utilities|Array|MakeArray "Point de problèmes. Je suis convaincu que tes pas te guideront à nouveau vers moi, vas cher apothicaire !") false self))
  (UserInterface|Viewport|AddtoViewport _returnvalue 0))

(fn ConstructionScript
  (|CallParentFunction))

(fn GetContent
  (bind _line (Variables|Default|Getline))
  (bind _line_2 (Variables|Default|Getline))
  (bind _line_3 (Variables|Default|Getline))
  (bind _line_4 (Variables|Default|Getline))
  (bind _sick_people (Variables|Default|Getsick%20people))
  (for _array_element (Variables|/Game/ThirdPerson/Blueprints/BP_ThirdPersonGameMode.BP_ThirdPersonGameMode_C|GetNPCs (Variables|Default|GetAs%20BP%20Third%20Person%20Game%20Mode))
    (if (Variables|/Game/Dev/Story/BP_Chara_Parent.BP_Chara_Parent_C|GetIsSick _array_element)
      (Math|Integer|IncrementInt (LocalVariables|Gettkt)
        (:%20%20
          (if (Utilities|Enum|Equal(Enum) (Variables|Default|GetText_line) "")
            (Variables|Default|SetText_line (Utilities|String|Append (Variables|/Game/Dev/Story/BP_Chara_Parent.BP_Chara_Parent_C|GetChara_name _array_element) " " "est malade"))
            (else
              (Variables|Default|SetText_line (Utilities|String|Append (Variables|Default|GetText_line) " 
" (Variables|/Game/Dev/Story/BP_Chara_Parent.BP_Chara_Parent_C|GetChara_name _array_element) " " "est malade."))))
          (if (>= (LocalVariables|Getmax_per_dialogue) 2)
            (LocalVariables|Setmax_per_dialogue 0)
            (Utilities|Array|SetArrayElem (Variables|Default|Getsick%20people) _line_2 (Variables|Default|GetText_line) true)
            (Utilities|Array|SetArrayElem (Variables|Default|GetNew_names) _line_2 (Variables|Default|GetChara_name) true)
            (Variables|Default|SetText_line "")
            (Math|Integer|IncrementInt (Variables|Default|Getline))
            (else
              (Math|Integer|IncrementInt (LocalVariables|Getmax_per_dialogue))))))))
  (if (== 0 (LocalVariables|Gettkt))
    (Utilities|Array|SetArrayElem _sick_people _line_4 "Hmmmm, j'ai bien l'impression que personne n'est malade. Réjouissons nous ! " true)
    (Utilities|Array|SetArrayElem (Variables|Default|GetNew_names) _line_4 (Variables|Default|GetChara_name) true)
    (elif (<= (LocalVariables|Getmax_per_dialogue) 2)
      (Utilities|Array|SetArrayElem (Variables|Default|Getsick%20people) _line (Variables|Default|GetText_line) true)
      (Utilities|Array|SetArrayElem (Variables|Default|GetNew_names) _line (Variables|Default|GetChara_name) true)
      (Variables|Default|SetText_line "")
      (bind _result (Math|Integer|IncrementInt (Variables|Default|Getline))
        (:%20%20
          (Utilities|Array|SetArrayElem (Variables|Default|Getsick%20people) _result "Voilà pour les personnes malades à Eudépar, n'hésite pas à me consulter à nouveau au besoin ! " true)
          (Utilities|Array|SetArrayElem (Variables|Default|GetNew_names) _result (Variables|Default|GetChara_name) true)))
      (else
        (Utilities|Array|SetArrayElem _sick_people _line_3 "Voilà pour les personnes malades à Eudépar, n'hésite pas à me consulter à nouveau au besoin ! " true)
        (Utilities|Array|SetArrayElem (Variables|Default|GetNew_names) _line_3 (Variables|Default|GetChara_name) true)))))