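; BP_Marc is a story NPC who asks the player for money to rebuild a bridge.
; A dialog choice shows the money widget, then either declines politely or checks that the player has at least 30.
; Payment updates the quest, displays the money change and swaps his dialog to shopkeeper greetings.
; The post-dialog event plays a black transition, teleports Marc, reveals the bridge and destroys the letter and blockers.
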(event EventBeginPlay
  (|CallParentFunction) ; This node is disabled and will not be called.\nDrag off pins to build functionality.
)

(event Collision|EventActorBeginOverlap
  (params (OtherActor :type Actor%20Object%20Reference))
  (|CallParentFunction OtherActor) ; This node is disabled and will not be called.\nDrag off pins to build functionality.
)

(event EventTick
  (params (DeltaSeconds :type Float%20%28single-precision%29))
  (|CallParentFunction DeltaSeconds) ; This node is disabled and will not be called.\nDrag off pins to build functionality.
)

(event EventUpperChoice
  (params (Widget :type WB%20Dialog%20System%20Object%20Reference))
  (CallFunction|CheckPlayerMoney Widget))

(event EventBottomChoice
  (params (Widget :type WB%20Dialog%20System%20Object%20Reference))
  (Widget|RemovefromParent Widget)
  (bind _returnvalue (UserInterface|CreateWidget "/Game/UI/Story/WB_Dialog_system.WB_Dialog_system_C" 0 (Utilities|Array|MakeArray "Marc") (Utilities|Array|MakeArray "C'est pas grave ptit gars, rien ne te force à dépenser ton argent pour ça.") false self))
  (UserInterface|Viewport|AddtoViewport _returnvalue 0)
  (Widget|RemovefromParent (Variables|Default|GetWidget_0)))

(event EventPostDialogEvent
  (bind _returnvalue (UserInterface|CreateWidget "/Game/UI/WB_Transi_Black.WB_Transi_Black_C"))
  (UserInterface|Viewport|AddtoViewport _returnvalue 0)
  (Utilities|FlowControl|Delay 1.2)
  (Transformation|SetWorldLocation (Variables|Default|GetCapsuleComponent) (Transformation|GetWorldLocation (Variables|/Game/Dev/BP_Tp_Ref.BP_Tp_Ref_C|GetDefaultSceneRoot (Variables|Default|GetTP))) false false)
  (Actor|DestroyActor (Variables|Default|Getlettre))
  (Rendering|SetActorHiddenInGame (Variables|Default|GetPont) false)
  (Actor|DestroyActor (Variables|Default|GetBlocking))
  (Actor|DestroyActor (Variables|Default|GetBlocking1)))

(event EventChoiceAppaearEvent
  (bind _returnvalue (UserInterface|CreateWidget "/Game/UI/WB_Money_Changes.WB_Money_Changes_C"))
  (Variables|Default|SetWidget_0 _returnvalue)
  (UserInterface|Viewport|AddtoViewport _returnvalue 0))

(fn ConstructionScript
  (|CallParentFunction))

(fn CheckPlayerMoney
  (params (NewParam :type WB%20Dialog%20System%20Object%20Reference))
  (if (>= (Variables|/Game/ThirdPerson/Blueprints/BP_ThirdPersonCharacter.BP_ThirdPersonCharacter_C|GetMoney (Variables|Default|GetAs%20BP%20Third%20Person%20Character)) 30)
    (CallFunction|QuestInits false)
    (Widget|RemovefromParent NewParam)
    (bind _returnvalue (UserInterface|CreateWidget "/Game/UI/Story/WB_Dialog_system.WB_Dialog_system_C" 0 (Utilities|Array|MakeArray "Marc" "Marc") (Utilities|Array|MakeArray "Merci pour ton aide !" "Grâce à tout ça, je vais pouvoir reconstruire le pont en un rien de temps, allez gop, au boulot ! ") false self false true))
    (UserInterface|Viewport|AddtoViewport _returnvalue 0)
    (Utilities|FlowControl|Sequence
      (:then_0
        (Variables|Default|SetPost_dialog_choice? false))
      (:then_1
        (Variables|Default|SetContents (Utilities|Array|MakeArray "Bienvenue petit gars, c'est gentil de passer !" "Prends ton temps pour regarder tous les articles !")))
      (:then_2
        (Variables|Default|SetNames (Utilities|Array|MakeArray "NewEnumerator1" "NewEnumerator1")))
      (:then_3
        (CallFunction|ConvertNames))
      (:then_4
        (Widget|RemovefromParent (Variables|Default|GetWidget_0))
        (Utilities|Platform|CollectGarbage))
      (:then_5
        (bind _returnvalue_2 (UserInterface|CreateWidget "/Game/UI/WB_Money_Changes.WB_Money_Changes_C" 0 false 30))
        (UserInterface|Viewport|AddtoViewport _returnvalue_2 0)
        (Default|OperateChange _returnvalue_2)))
    (else
      (Widget|RemovefromParent NewParam)
      (bind _returnvalue_3 (UserInterface|CreateWidget "/Game/UI/Story/WB_Dialog_system.WB_Dialog_system_C" 0 (Utilities|Array|MakeArray "Marc") (Utilities|Array|MakeArray "Je suis désolé mon petit, mais même avec tout ton argent, ce n'est pas suffisant...") false self))
      (UserInterface|Viewport|AddtoViewport _returnvalue_3 0)
      (Widget|RemovefromParent (Variables|Default|GetWidget_0)))))