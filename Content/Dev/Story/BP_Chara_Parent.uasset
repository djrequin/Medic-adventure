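; Parent Blueprint for story NPCs that can talk to the player, show a quest marker and fall sick.
; It registers with the game mode, and interacting optionally turns it toward the player and opens a dialog widget with healthy or sick lines.
; Disease functions set HP, tries and rank, boost damage on a weakness match, and end sickness when HP or tries run out.
; Choice and post-dialog events are empty hooks.
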(event Custom|choice_appaear_event)

(event Custom|Post_Dialog_event)

(event Custom|Upper_choice
  (params (Widget :type WB%20Dialog%20System%20Object%20Reference)))

(event Custom|Bottom%20choice
  (params (Widget :type WB%20Dialog%20System%20Object%20Reference)))

(event Custom|reset%20rotation
  (if (Variables|Default|GetTurn%20to%20player?)
    (Transformation|SetWorldRotation (Variables|Collision|GetCapsuleComponent) (Variables|Default|Getbase_rota) false false)))

(event EventBeginPlay
  (Variables|Default|Setbase_rota (Transformation|GetActorRotation))
  (Variables|Default|SetEntry_text "Parler")
  (CallFunction|ConvertNames)
  (Rendering|SetVisibility (Variables|Default|GetSick_Ping) false false)
  (bind _asbp_third_person_game_mode (Utilities|Casting|CastToBP_ThirdPersonGameMode (Game|GetGameMode)))
  (bind _output_get (Variables|Default|SetAs%20BP%20Third%20Person%20Game%20Mode _asbp_third_person_game_mode))
  (Utilities|Array|Add (Variables|/Game/ThirdPerson/Blueprints/BP_ThirdPersonGameMode.BP_ThirdPersonGameMode_C|GetNPCs _output_get) self)
  (Variables|Default|SetChara_name (Utilities|String|EnumtoString (Variables|Default|GetName)))
  (bind _asbp_third_person_character (Utilities|Casting|CastToBP_ThirdPersonCharacter (Game|GetPlayerCharacter 0)))
  (Variables|Default|SetAs%20BP%20Third%20Person%20Character _asbp_third_person_character)
  (CallFunction|QuestInits (Variables|Default|GetHas_a_quest?)))

(event Collision|EventActorBeginOverlap
  (params (OtherActor :type Actor%20Object%20Reference)))

(event EventTick
  (params (DeltaSeconds :type Float%20%28single-precision%29)))

(event EventPrintInteractionButton
  (params (Widget :type WB%20Interaction%20Button%20Object%20Reference))
  (Default|Print Widget (Variables|Default|GetEntry_text)))

(event EventInteraction
  (bind _base_rota (Variables|Default|Getbase_rota))
  (if (Variables|Default|GetCan_talk%20?)
    (if (Variables|Default|GetTurn%20to%20player?)
      (Transformation|SetWorldRotation (Variables|Collision|GetCapsuleComponent) (Math|Rotator|MakeRotator (.roll _base_rota) (.pitch _base_rota) (.yaw (Math|Rotator|FindLookatRotation (Transformation|GetActorLocation) (Transformation|GetActorLocation (Game|GetPlayerCharacter 0))))) false false))
    (if (Variables|Disease|GetIsSick)
      (bind _returnvalue (UserInterface|CreateWidget "/Game/UI/Story/WB_Dialog_system.WB_Dialog_system_C" 0 (Variables|Default|GetSick%20names) (Variables|Default|GetSick%20Content) (Variables|Disease|GetIsSick) self (Variables|Default|GetPost_dialog_choice?) (Variables|Default|GetPost_dialog_event?)))
      (UserInterface|Viewport|AddtoViewport _returnvalue 0)
      (else
        (bind _returnvalue_2 (UserInterface|CreateWidget "/Game/UI/Story/WB_Dialog_system.WB_Dialog_system_C" 0 (Variables|Default|GetH_Names) (Variables|Default|GetContents) (Variables|Disease|GetIsSick) self (Variables|Default|GetPost_dialog_choice?) (Variables|Default|GetPost_dialog_event?)))
        (UserInterface|Viewport|AddtoViewport _returnvalue_2 0)))))

(fn ConstructionScript)

(fn ConvertNames
  (for _array_element (Variables|Default|GetNames)
    (Utilities|Array|Add (Variables|Default|GetH_Names) (Utilities|String|EnumtoString _array_element)))
  (for _array_element_2 (Variables|Default|GetSick%20name)
    (Utilities|Array|Add (Variables|Default|GetSick%20names) (Utilities|String|EnumtoString _array_element_2))))

(fn InitializeDisease
  (params (Disease_Type :type Enum_Diseases%20Enum :default "Enum_Diseases_MAX") (HP :type Float%20%28double-precision%29) (Try :type Integer) (Rank :type Enum_ranks%20Enum :default "NewEnumerator0"))
  (Variables|Disease|SetDisease%20Type Disease_Type)
  (bind _output_get (Variables|Disease|SetD_HP%20Max HP))
  (Variables|Disease|SetD_Current_HP _output_get)
  (Variables|Disease|SetD_Try Try)
  (Variables|Disease|SetD_Rank Rank)
  (Variables|Disease|SetIsSick true)
  (Rendering|SetVisibility (Variables|Default|GetSick_Ping) true false))

(fn DamageMultiplier
  (params (Efficiency :type Float%20%28double-precision%29) (Weakness :type Enum_Diseases%20Enum :default "NewEnumerator0"))
  (LocalVariables|SetDamages%20dealt Efficiency)
  (if (Utilities|Enum|Equal(Enum) Weakness (Variables|Disease|GetDisease%20Type))
    (LocalVariables|SetDamages%20dealt (* (LocalVariables|GetDamages%20dealt) 1.5))
    (LocalVariables|SetEffective? true))
  (return (LocalVariables|GetDamages%20dealt) (LocalVariables|GetEffective?)))

(fn TakeDamages
  (params (Damages :type Float%20%28double-precision%29) (Was_effective? :type Boolean) (Widget :type WB%20Sickness%20Object%20Reference))
  (LocalVariables|SetWasEffective Was_effective?)
  (Default|ReduceHp Widget Damages)
  (bind _output_get (Variables|Disease|SetD_Current_HP (Math|Float|Clamp(Float) (- (Variables|Disease|GetD_Current_HP) Damages) 0.0 (Variables|Disease|GetD_HP%20Max))))
  (if (<= _output_get 0.0)
    (Development|PrintString "Healed !")
    (Variables|Disease|SetIsSick false)
    (LocalVariables|SetHealed true)
    (else
      (LocalVariables|SetHealed false)
      (bind _result (Math|Integer|DecrementInt (Variables|Disease|GetD_Try))
        (:%20%20
          (if (<= _result 0)
            (Variables|Disease|SetIsSick false)
            (LocalVariables|SetFail true))))))
  (return (Variables|Disease|GetD_Rank) (Variables|Disease|GetD_HP%20Max) (LocalVariables|GetHealed) (LocalVariables|GetWasEffective) (LocalVariables|GetFail) (Variables|Disease|GetD_Try)))

(fn QuestInits
  (params (show? :type Boolean))
  (if show?
    (Rendering|SetVisibility (Variables|Default|GetQuest_ping) true false)
    (else
      (Rendering|SetVisibility (Variables|Default|GetQuest_ping) false false))))