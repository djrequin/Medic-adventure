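; BP_Pak is a story character that answers a two-option dialogue choice with French lines about the Guéritou healing herb.
; UpperChoice and BottomChoice each remove the passed-in widget, then open a WB_Dialog_system widget showing CharaName and a hard-coded reply.
; The upper reply praises Pak's own herb, while the lower one points to the O'vertige mountain to find one.
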(event EventBeginPlay
  (|CallParentFunction) ; This node is disabled and will not be called.\nDrag off pins to build functionality.
)

(event Collision|EventActorBeginOverlap
  (params (OtherActor :type Actor%20Object%20Reference))
  (|CallParentFunction OtherActor) ; This node is disabled and will not be called.\nDrag off pins to build functionality.
)

(event EventTick
  (params (DeltaSeconds :type Float%20%28single-precision%29))
  (|CallParentFunction DeltaSeconds) ; This node is disabled and will not be called.\nDrag off pins to build functionality.
)

(event EventUpperChoice
  (params (Widget :type WB%20Dialog%20System%20Object%20Reference))
  (Widget|RemovefromParent Widget)
  (bind _returnvalue (UserInterface|CreateWidget "/Game/UI/Story/WB_Dialog_system.WB_Dialog_system_C" 0 (Utilities|Array|MakeArray (Variables|Default|GetChara_name)) (Utilities|Array|MakeArray "Mon herbe Guéritou est plus efficace que la moyenne. Je n'en ai jamais vu une aussi efficace de ma vie. ") false 0))
  (UserInterface|Viewport|AddtoViewport _returnvalue 0))

(event EventBottomChoice
  (params (Widget :type WB%20Dialog%20System%20Object%20Reference))
  (Widget|RemovefromParent Widget)
  (bind _returnvalue (UserInterface|CreateWidget "/Game/UI/Story/WB_Dialog_system.WB_Dialog_system_C" 0 (Utilities|Array|MakeArray (Variables|Default|GetChara_name)) (Utilities|Array|MakeArray "Si tu veux une herbe Guéritou, tu n'as qu'à aller en chercher une dans la montagne O'vertige.") false 0))
  (UserInterface|Viewport|AddtoViewport _returnvalue 0))

(fn ConstructionScript
  (|CallParentFunction))