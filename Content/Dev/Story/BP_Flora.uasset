(event Custom|Walked_flower
  (Utilities|FlowControl|DoOnce false
    (:Completed
      (bind _returnvalue (UserInterface|CreateWidget "/Game/UI/Story/WB_Dialog_system.WB_Dialog_system_C" 0 (Utilities|Array|MakeArray (Variables|Default|GetChara_name)) (Utilities|Array|MakeArray "Raaaaaaah, non, il ne faut pas marcher sur les fleurs !!!! Reviens ici !") false self false true))
      (UserInterface|Viewport|AddtoViewport _returnvalue 0))))

(event Custom|check_ingredients
  (bind _returnvalue (Utilities|Time|SetTimerbyEvent (delegate Custom|check_ings) 0.5 true))
  (Variables|Default|Settimer _returnvalue))

(event Custom|check_ings
  (bind _chara_name (Variables|Default|GetChara_name))
  (bind _chara_name_2 (Variables|Default|GetChara_name))
  (for _array_element (Variables|Default|GetIngredients)
    (Utilities|IsValid _array_element
      (:Is%20Not%20Valid
        (Math|Integer|IncrementInt (Variables|Default|Getget_numbers)
          (:%20%20
            (bind _returnvalue (Utilities|Array|RemoveItem (Variables|Default|GetIngredients) _array_element))
            (Development|PrintString (Utilities|String|ToString(Boolean) _returnvalue)))))))
  (if (>= (Variables|Default|Getget_numbers) (Variables|Default|Geting_number))
    (Utilities|Time|ClearandInvalidateTimerbyHandle (Variables|Default|Gettimer))
    (bind _returnvalue_2 (UserInterface|CreateWidget "/Game/UI/Story/WB_Dialog_system.WB_Dialog_system_C" 0 (Utilities|Array|MakeArray _chara_name_2 _chara_name_2) (Utilities|Array|MakeArray "Oh tu les as tous ramassés, merci infiniment !" "Reviens ici avec précaution ! Bien sûr, même si tu as tout ramassé, ça ne veut pas dire que je t'autoriserais à marcher dessus à l'avenir.") false self false true))
    (UserInterface|Viewport|AddtoViewport _returnvalue_2 0)
    (CallFunction|QuestInits false)
    (Utilities|FlowControl|Sequence
      (:then_0
        (Variables|Default|SetPost_dialog_choice? false))
      (:then_1
        (Variables|Default|SetContents (Utilities|Array|MakeArray "Tu m'as bien aidée, merci beaucoup ! Tu es très agile, peut-être grâce à ton âge. Mais en tout cas, merci infiniment !" "Bien  sûr, cela ne veut pas dire que tu auras le droit de marcher sur mes fleurs à l'avenir.")))
      (:then_2
        (Variables|Default|SetH_Names (Utilities|Array|MakeArray _chara_name _chara_name))))))

(event EventBeginPlay
  (|CallParentFunction)
  (CallFunction|SetVariables)
  (bind _output_get (Variables|Default|Seting_number (Utilities|Array|Length (Variables|Default|GetIngredients))))
  (Development|PrintString (Utilities|String|ToString(Integer) _output_get))
  (CallFunction|CheckIngredients))

(event Collision|EventActorBeginOverlap
  (params (OtherActor :type Actor%20Object%20Reference))
  (|CallParentFunction OtherActor) ; This node is disabled and will not be called.\nDrag off pins to build functionality.
)

(event EventTick
  (params (DeltaSeconds :type Float%20%28single-precision%29))
  (|CallParentFunction DeltaSeconds) ; This node is disabled and will not be called.\nDrag off pins to build functionality.
)

(event EventUpperChoice
  (params (Widget :type WB%20Dialog%20System%20Object%20Reference))
  (Widget|RemovefromParent Widget)
  (bind _returnvalue (UserInterface|CreateWidget "/Game/UI/Story/WB_Dialog_system.WB_Dialog_system_C" 0 (Utilities|Array|MakeArray (Variables|Default|GetChara_name)) (Utilities|Array|MakeArray "Super ! Je compte sur toi !") false self))
  (UserInterface|Viewport|AddtoViewport _returnvalue 0))

(event EventBottomChoice
  (params (Widget :type WB%20Dialog%20System%20Object%20Reference))
  (Widget|RemovefromParent Widget)
  (bind _returnvalue (UserInterface|CreateWidget "/Game/UI/Story/WB_Dialog_system.WB_Dialog_system_C" 0 (Utilities|Array|MakeArray (Variables|Default|GetChara_name)) (Utilities|Array|MakeArray "Oh, je comprends...") false self))
  (UserInterface|Viewport|AddtoViewport _returnvalue 0))

(event EventPostDialogEvent
  (bind _as_bp_third_person_character (Variables|Default|GetAs%20BP%20Third%20Person%20Character))
  (bind _tp_point (Variables|Default|GetTP_point))
  (bind _capsulecomponent (Variables|/Script/Engine.Character|GetCapsuleComponent _as_bp_third_person_character))
  (bind _returnvalue (UserInterface|CreateWidget "/Game/UI/WB_Transi_Black.WB_Transi_Black_C"))
  (UserInterface|Viewport|AddtoViewport _returnvalue 0)
  (Utilities|FlowControl|Delay 1.2)
  (Transformation|SetWorldLocation _capsulecomponent (Transformation|GetActorLocation _tp_point) false false)
  (Transformation|SetWorldRotation _capsulecomponent (Transformation|GetActorRotation _tp_point) false false)
  (for _array_element (Variables|Default|GetBoxes)
    (Default|ResetEvent _array_element))
  (Utilities|FlowControl|DoOnce false) ; enters at Reset
)

(fn ConstructionScript
  (|CallParentFunction))

(fn SetVariables
  (for _array_element (Variables|Default|GetBoxes)
    (Variables|/Game/Dev/BP_Mini_game.BP_Mini_game_C|SetFlora _array_element self)))