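; BP_Chaudron is a cauldron where the player combines an ingredient and a catalyst into a medicine.
; Interaction stores the held ingredient if its slot is empty, otherwise the held catalyst, then checks whether both are present.
; ConstructMedic averages their efficiencies, taking type from the catalyst, target disease from the ingredient and name from both.
; The new BP_Medicament joins the player's Medocs list, and the cauldron and hand slots clear.
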(event Custom|Final_check
  (Utilities|IsValid (Variables|Default|GetCatalyst)
    (:Is%20Valid
      (Utilities|IsValid (Variables|Default|GetIng)
        (:Is%20Valid
          (bind _returnvalue (Game|ConstructObjectfromClass "/Game/ThirdPerson/Blueprints/BP_Medicament.BP_Medicament_C" (.efficiency (CallFunction|ConstructMedic (Variables|Default|GetCatalyst) (Variables|Default|GetIng))) (.Type (CallFunction|ConstructMedic (Variables|Default|GetCatalyst) (Variables|Default|GetIng))) (.Effective%20disease (CallFunction|ConstructMedic (Variables|Default|GetCatalyst) (Variables|Default|GetIng))) (.Name (CallFunction|ConstructMedic (Variables|Default|GetCatalyst) (Variables|Default|GetIng)))))
          (Default|InitImage _returnvalue)
          (Utilities|Array|Add (Variables|/Game/ThirdPerson/Blueprints/BP_ThirdPersonCharacter.BP_ThirdPersonCharacter_C|GetMedocs (stale EventInteraction _asbp_third_person_character)) _returnvalue)
          (Development|PrintString (Variables|/Game/ThirdPerson/Blueprints/BP_Medicament.BP_Medicament_C|GetName _returnvalue))
          (Variables|Default|SetCatalyst 0)
          (Variables|Default|SetIng 0)
          (Variables|/Game/ThirdPerson/Blueprints/BP_ThirdPersonCharacter.BP_ThirdPersonCharacter_C|SetIn_Hand_catalyst (stale EventInteraction _asbp_third_person_character) 0)
          (Variables|/Game/ThirdPerson/Blueprints/BP_ThirdPersonCharacter.BP_ThirdPersonCharacter_C|SetIn_Hand_Ingredient (stale EventInteraction _asbp_third_person_character) 0))))))

(event EventBeginPlay
  (|CallParentFunction) ; This node is disabled and will not be called.\nDrag off pins to build functionality.
)

(event Collision|EventActorBeginOverlap
  (params (OtherActor :type Actor%20Object%20Reference))
  (|CallParentFunction OtherActor) ; This node is disabled and will not be called.\nDrag off pins to build functionality.
)

(event EventTick
  (params (DeltaSeconds :type Float%20%28single-precision%29))
  (|CallParentFunction DeltaSeconds) ; This node is disabled and will not be called.\nDrag off pins to build functionality.
)

(event EventInteraction
  (bind _asbp_third_person_character (Utilities|Casting|CastToBP_ThirdPersonCharacter (Game|GetPlayerCharacter 0)))
  (Utilities|IsValid (Variables|/Game/ThirdPerson/Blueprints/BP_ThirdPersonCharacter.BP_ThirdPersonCharacter_C|GetIn_Hand_Ingredient _asbp_third_person_character)
    (:Is%20Valid
      (Utilities|IsValid (Variables|Default|GetIng)
        (:Is%20Valid
          (Utilities|IsValid (Variables|/Game/ThirdPerson/Blueprints/BP_ThirdPersonCharacter.BP_ThirdPersonCharacter_C|GetIn_Hand_catalyst _asbp_third_person_character) :!label _label
            (:Is%20Valid
              (Variables|Default|SetCatalyst (Variables|/Game/ThirdPerson/Blueprints/BP_ThirdPersonCharacter.BP_ThirdPersonCharacter_C|GetIn_Hand_catalyst _asbp_third_person_character)))))
        (:Is%20Not%20Valid
          (Variables|Default|SetIng (Variables|/Game/ThirdPerson/Blueprints/BP_ThirdPersonCharacter.BP_ThirdPersonCharacter_C|GetIn_Hand_Ingredient _asbp_third_person_character)))))
    (:Is%20Not%20Valid
      (goto _label)))
  (CallFunction|FinalCheck))

(fn ConstructionScript
  (|CallParentFunction))

(fn ConstructMedic
  (params (Catalyst :type BP%20Ingredient%20Object%20Reference) (Ing :type BP%20Ingredient%20Object%20Reference))
  (bind _catalyst_type (Variables|/Game/Dev/Collectibles/BP_Ingredient.BP_Ingredient_C|GetCatalyst_type Catalyst))
  (return (/ (+ (Variables|/Game/Dev/Collectibles/BP_Ingredient.BP_Ingredient_C|GetEfficiency Catalyst) (Variables|/Game/Dev/Collectibles/BP_Ingredient.BP_Ingredient_C|GetEfficiency Ing)) 2) _catalyst_type (Variables|/Game/Dev/Collectibles/BP_Ingredient.BP_Ingredient_C|GetEffective%20disease Ing) (Utilities|String|Append (Utilities|String|EnumtoString _catalyst_type) " " (Variables|/Game/Dev/Collectibles/BP_Ingredient.BP_Ingredient_C|GetAcronyme Ing))))