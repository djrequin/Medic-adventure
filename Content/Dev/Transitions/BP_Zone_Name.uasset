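; BP_Zone_Name is a trigger zone that changes the soundtrack and announces a location name when the third-person character enters.
; Box overlap asks BP_ThirdPersonGameMode to switch to the zone's AssociatedOst on every entry.
; A DoOnce gates creation of the WB_Village_anouncement widget showing CityName, and a delayed custom event re-arms it after a minute so the announcement does not repeat on quick re-entry.
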(event OnComponentBeginOverlap(Box)
  (params (OverlappedComponent :type Primitive%20Component%20Object%20Reference) (OtherActor :type Actor%20Object%20Reference) (OtherComp :type Primitive%20Component%20Object%20Reference) (OtherBodyIndex :type Integer) (bFromSweep :type Boolean) (SweepResult :type Hit%20Result%20Structure%20%28by%20ref%29))
  (Utilities|Casting|CastToBP_ThirdPersonCharacter OtherActor)
  (Default|ChangeOst (.AsBP%20Third%20Person%20Game%20Mode (Utilities|Casting|CastToBP_ThirdPersonGameMode (Game|GetGameMode))) (Variables|Default|GetAssociated_ost))
  (Utilities|FlowControl|DoOnce false
    (:Completed
      (CallFunction|Delay)
      (bind _returnvalue (UserInterface|CreateWidget "/Game/UI/UX/WB_Village_anouncement.WB_Village_anouncement_C" 0 (Variables|Default|GetCity%20Name)))
      (UserInterface|Viewport|AddtoViewport _returnvalue 0))))

(event Custom|Delay
  (Utilities|FlowControl|Delay 6e+01)
  (Utilities|FlowControl|DoOnce false) ; enters at Reset
)

(event EventBeginPlay)

(event Collision|EventActorBeginOverlap
  (params (OtherActor :type Actor%20Object%20Reference)))

(event EventTick
  (params (DeltaSeconds :type Float%20%28single-precision%29)))

(fn ConstructionScript)