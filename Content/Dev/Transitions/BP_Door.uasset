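; Interactable transition door that swings open and teleports the third-person player to a referenced spawn point.
; Interaction disables player input, runs a forward rotator for a timed swing and shows the WB_Fade widget.
; Partway through the swing, it moves and reorients the player's capsule at the spawn point, starts the timed reverse rotator and restores input.
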(event Custom|Door_opening
  (bind _forward_rotator (Variables|Default|GetForward_rotator))
  (bind _spawn_point (Variables|Default|GetSpawn_point))
  (bind _as_bp_third_person_character (Variables|Default|GetAs%20BP%20Third%20Person%20Character))
  (bind _capsulecomponent (Variables|/Script/Engine.Character|GetCapsuleComponent _as_bp_third_person_character))
  (bind _ref (Variables|/Game/Dev/Transitions/BP_exit.BP_exit_C|Getref _spawn_point))
  (bind _returnvalue (Transformation|GetWorldRotation _ref))
  (Utilities|FlowControl|Sequence
    (:then_0
      (Input|DisableInput (Variables|Default|GetAs%20BP%20Third%20Person%20Character) (Game|GetPlayerController 0))
      (Components|Activation|Activate _forward_rotator false)
      (Utilities|FlowControl|Delay 1.0)
      (Components|Activation|Deactivate _forward_rotator))
    (:then_1
      (bind _returnvalue_2 (UserInterface|CreateWidget "/Game/UI/UX/WB_Fade.WB_Fade_C"))
      (UserInterface|Viewport|AddtoViewport _returnvalue_2 0))
    (:then_2
      (Utilities|FlowControl|Delay 0.5)
      (Transformation|SetWorldLocation _capsulecomponent (Transformation|GetWorldLocation _ref) false false)
      (Transformation|SetWorldRotation _capsulecomponent (Math|Rotator|MakeRotator (.roll _returnvalue) (- (.pitch _returnvalue) 1.8e+02) (.yaw _returnvalue)) false false)
      (CallFunction|ReverseOpening)
      (Input|EnableInput (Variables|Default|GetAs%20BP%20Third%20Person%20Character) (Game|GetPlayerController 0)))))

(event Custom|Reverse_opening
  (bind _reverse_rotator (Variables|Default|GetReverse_rotator))
  (Components|Activation|Activate _reverse_rotator false)
  (Utilities|FlowControl|Delay 1.0)
  (Components|Activation|Deactivate _reverse_rotator))

(event EventBeginPlay
  (|CallParentFunction)
  (bind _asbp_third_person_character (Utilities|Casting|CastToBP_ThirdPersonCharacter (Game|GetPlayerCharacter 0)))
  (Variables|Default|SetAs%20BP%20Third%20Person%20Character _asbp_third_person_character))

(event Collision|EventActorBeginOverlap
  (params (OtherActor :type Actor%20Object%20Reference))
  (|CallParentFunction OtherActor) ; This node is disabled and will not be called.\nDrag off pins to build functionality.
)

(event EventTick
  (params (DeltaSeconds :type Float%20%28single-precision%29))
  (|CallParentFunction DeltaSeconds) ; This node is disabled and will not be called.\nDrag off pins to build functionality.
)

(event EventInteraction
  (CallFunction|DoorOpening))

(fn ConstructionScript
  (|CallParentFunction))