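; BP_exit is a transition trigger that moves the third-person player character to a spawn point behind a screen fade.
; When the character overlaps its Box, it disables input and adds a WB_Fade widget to the viewport.
; After a half-second delay, it sets the capsule's world location to the SpawnPoint reference's location and re-enables input.
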(event OnComponentBeginOverlap(Box)
  (params (OverlappedComponent :type Primitive%20Component%20Object%20Reference) (OtherActor :type Actor%20Object%20Reference) (OtherComp :type Primitive%20Component%20Object%20Reference) (OtherBodyIndex :type Integer) (bFromSweep :type Boolean) (SweepResult :type Hit%20Result%20Structure%20%28by%20ref%29))
  (bind _asbp_third_person_character (Utilities|Casting|CastToBP_ThirdPersonCharacter OtherActor))
  (Input|DisableInput _asbp_third_person_character (Game|GetPlayerController 0))
  (Utilities|FlowControl|Sequence
    (:then_0
      (bind _returnvalue (UserInterface|CreateWidget "/Game/UI/UX/WB_Fade.WB_Fade_C"))
      (UserInterface|Viewport|AddtoViewport _returnvalue 0))
    (:then_1
      (Utilities|FlowControl|Delay 0.5)
      (Transformation|SetWorldLocation (Variables|/Script/Engine.Character|GetCapsuleComponent _asbp_third_person_character) (Transformation|GetWorldLocation (Variables|/Game/Dev/Transitions/BP_Door.BP_Door_C|Getref (Variables|Default|GetSpawn_Point))) false false)
      (Input|EnableInput _asbp_third_person_character (Game|GetPlayerController 0)))))

(event EventBeginPlay)

(event Collision|EventActorBeginOverlap
  (params (OtherActor :type Actor%20Object%20Reference)))

(event EventTick
  (params (DeltaSeconds :type Float%20%28single-precision%29)))

(fn ConstructionScript)