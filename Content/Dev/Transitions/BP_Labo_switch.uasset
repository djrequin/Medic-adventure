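; Trigger volume for the potion-crafting lab that shows the recipe UI while the player stands inside its box.
; Entering creates a WB_Recipe widget linked to the Chaudron (cauldron), and leaving removes it, forces garbage collection and resets the gate.
; A second, never-reset DoOnce shows a French illustrated tutorial on concoctions on first entry only.
; On BeginPlay it adds itself to the player character's IgnoreTrace list.
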(event OnComponentBeginOverlap(Box)
  (params (OverlappedComponent :type Primitive%20Component%20Object%20Reference) (OtherActor :type Actor%20Object%20Reference) (OtherComp :type Primitive%20Component%20Object%20Reference) (OtherBodyIndex :type Integer) (bFromSweep :type Boolean) (SweepResult :type Hit%20Result%20Structure%20%28by%20ref%29))
  (Utilities|Casting|CastToBP_ThirdPersonCharacter OtherActor)
  (Utilities|FlowControl|DoOnce false
    (:Completed
      (bind _returnvalue (UserInterface|CreateWidget "/Game/UI/WB_Recipe.WB_Recipe_C" 0 (Variables|Default|GetChaudron)))
      (bind _output_get (Variables|Default|SetWidget _returnvalue))
      (Variables|/Game/Dev/BP_Chaudron.BP_Chaudron_C|Setwidg (Variables|Default|GetChaudron) _output_get)
      (UserInterface|Viewport|AddtoViewport _output_get 0)
      (Utilities|FlowControl|DoOnce false
        (:Completed
          (bind _returnvalue_2 (UserInterface|CreateWidget "/Game/UI/Tutorials/WB_Tutorials.WB_Tutorials_C" 0 (Utilities|Array|MakeArray "Afin de soigner les gens malades, il est essentiel de créer des concoctions.  
 
Ces dernières sont toujours constitutées d'un catalyseur trouvable dans les coffres rouges et d'un ingrédient à effet, rangé dans les coffres normaux." "Pour créer un médicament, rien de plus simple ! Il faut mélanger les deux ingrédients.  
Une fois sélectionnés, interagissez avec le chaudron et celui-ci finalisera la création ! 
Une fois que le chaudron a finalisé, la concoction est prête à être donnée." "Chaque catalyseur définit le type de concoction qui sera créée.  
 
Baies : Onguent 
Touffe : Pillule 
Coquillage : Sirop." "Les ingrédients normaux sont ceux qui combattront la maladie. Chaque ingrédient est efficace contre un type de symptôme.  
Par exemple, la plante Touss-Touss est efficace contre la toux. 
 
Pour connaître les efficacités, n'hésitez pas à lire les descriptions de la guilde. Celles-ci fourmillent d'informations. 
 
Cependant, pas d'inquiètude. Si un médicament pas efficace est donné à  un malade, celui-ci combattra tout de même la maladie !" "Pour reconnaître les gens malades, rien de plus simple ! Ceux-ci ont un signe distinctif !  
 
J'ai aussi cru entendre qu'un mentaliste capable de les détecter trainait dans le village...") (Utilities|Array|MakeArray "Concoctions" "1. Préparation" "2. Types" "3. Efficacités" "4. Malades") (Utilities|Array|MakeArray (Utilities|Struct|MakeSlateBrush "Image" "NoTile" "NoMirror" "(X=32.000000,Y=32.000000)" "(Left=0.000000,Top=0.000000,Right=0.000000,Bottom=0.000000)" "(SpecifiedColor=(R=1.000000,G=1.000000,B=1.000000,A=1.000000),ColorUseRule=UseColor_Specified)" "(CornerRadii=(X=0.000000,Y=0.000000,Z=0.000000,W=1.000000),Color=(SpecifiedColor=(R=0.000000,G=0.000000,B=0.000000,A=0.000000),ColorUseRule=UseColor_Specified),Width=0.000000,RoundingType=HalfHeightRadius,bUseBrushTransparency=False)" "/Game/UI/Tutorials/Images_ms/MS1.MS1") (Utilities|Struct|MakeSlateBrush "Image" "NoTile" "NoMirror" "(X=32.000000,Y=32.000000)" "(Left=0.000000,Top=0.000000,Right=0.000000,Bottom=0.000000)" "(SpecifiedColor=(R=1.000000,G=1.000000,B=1.000000,A=1.000000),ColorUseRule=UseColor_Specified)" "(CornerRadii=(X=0.000000,Y=0.000000,Z=0.000000,W=1.000000),Color=(SpecifiedColor=(R=0.000000,G=0.000000,B=0.000000,A=0.000000),ColorUseRule=UseColor_Specified),Width=0.000000,RoundingType=HalfHeightRadius,bUseBrushTransparency=False)" "/Game/UI/Tutorials/images_tuto/TS3.TS3") (Utilities|Struct|MakeSlateBrush "Image" "NoTile" "NoMirror" "(X=32.000000,Y=32.000000)" "(Left=0.000000,Top=0.000000,Right=0.000000,Bottom=0.000000)" "(SpecifiedColor=(R=1.000000,G=1.000000,B=1.000000,A=1.000000),ColorUseRule=UseColor_Specified)" "(CornerRadii=(X=0.000000,Y=0.000000,Z=0.000000,W=1.000000),Color=(SpecifiedColor=(R=0.000000,G=0.000000,B=0.000000,A=0.000000),ColorUseRule=UseColor_Specified),Width=0.000000,RoundingType=HalfHeightRadius,bUseBrushTransparency=False)" "/Game/Images/Sirop.Sirop") (Utilities|Struct|MakeSlateBrush "Image" "NoTile" "NoMirror" "(X=32.000000,Y=32.000000)" "(Left=0.000000,Top=0.000000,Right=0.000000,Bottom=0.000000)" "(SpecifiedColor=(R=1.000000,G=1.000000,B=1.000000,A=1.000000),ColorUseRule=UseColor_Specified)" "(CornerRadii=(X=0.000000,Y=0.000000,Z=0.000000,W=1.000000),Color=(SpecifiedColor=(R=0.000000,G=0.000000,B=0.000000,A=0.000000),ColorUseRule=UseColor_Specified),Width=0.000000,RoundingType=HalfHeightRadius,bUseBrushTransparency=False)" "/Game/Dev/Collectibles/Images/V2/Miel_toudou.Miel_toudou") (Utilities|Struct|MakeSlateBrush "Image" "NoTile" "NoMirror" "(X=32.000000,Y=32.000000)" "(Left=0.000000,Top=0.000000,Right=0.000000,Bottom=0.000000)" "(SpecifiedColor=(R=1.000000,G=1.000000,B=1.000000,A=1.000000),ColorUseRule=UseColor_Specified)" "(CornerRadii=(X=0.000000,Y=0.000000,Z=0.000000,W=1.000000),Color=(SpecifiedColor=(R=0.000000,G=0.000000,B=0.000000,A=0.000000),ColorUseRule=UseColor_Specified),Width=0.000000,RoundingType=HalfHeightRadius,bUseBrushTransparency=False)" "/Game/UI/Tutorials/Images_ms/MS2.MS2"))))
          (UserInterface|Viewport|AddtoViewport _returnvalue_2 0))))))

(event OnComponentEndOverlap(Box)
  (params (OverlappedComponent :type Primitive%20Component%20Object%20Reference) (OtherActor :type Actor%20Object%20Reference) (OtherComp :type Primitive%20Component%20Object%20Reference) (OtherBodyIndex :type Integer))
  (Utilities|Casting|CastToBP_ThirdPersonCharacter OtherActor)
  (Utilities|IsValid (Variables|Default|GetWidget)
    (:Is%20Valid
      (Widget|RemovefromParent (Variables|Default|GetWidget))
      (Utilities|Platform|CollectGarbage)
      (Utilities|FlowControl|DoOnce false) ; enters at Reset
    )))

(event EventBeginPlay
  (Utilities|Array|Add (Variables|/Game/ThirdPerson/Blueprints/BP_ThirdPersonCharacter.BP_ThirdPersonCharacter_C|Getignore_trace (.AsBP%20Third%20Person%20Character (Utilities|Casting|CastToBP_ThirdPersonCharacter (Game|GetPlayerCharacter 0)))) self))

(fn ConstructionScript)