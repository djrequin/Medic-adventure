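; Story trigger volume that updates the mayor (BP_Maire) with new dialogue when that actor overlaps its box.
; It copies its Content and Names to the mayor, calls ConvertNames, and optionally enables the tutorial flag.
; When flagged as Ending, it also destroys the listed actors and calls the mayor's Erreur with illustrated French pages welcoming the player to the apothecary guild and explaining its activities.
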(event OnComponentBeginOverlap(Box)
  (params (OverlappedComponent :type Primitive%20Component%20Object%20Reference) (OtherActor :type Actor%20Object%20Reference) (OtherComp :type Primitive%20Component%20Object%20Reference) (OtherBodyIndex :type Integer) (bFromSweep :type Boolean) (SweepResult :type Hit%20Result%20Structure%20%28by%20ref%29))
  (bind _asbp_maire (Utilities|Casting|CastToBP_Maire OtherActor))
  (Utilities|FlowControl|Sequence
    (:then_0
      (Variables|/Game/Dev/Story/BP_Chara_Parent.BP_Chara_Parent_C|SetContents _asbp_maire (Variables|Default|GetContent)))
    (:then_1
      (Variables|/Game/Dev/Story/BP_Chara_Parent.BP_Chara_Parent_C|SetNames _asbp_maire (Variables|Default|GetNames)))
    (:then_2
      (Default|ConvertNames _asbp_maire))
    (:then_3
      (if (Variables|Default|GetActivate_tuto%20?)
        (Variables|/Game/Dev/Story/BP_Maire.BP_Maire_C|Setactivate%20tuto%20? _asbp_maire true)))
    (:then_4
      (if (Variables|Default|Getending?)
        (for _array_element (Variables|Default|Getdestroys)
          (Actor|DestroyActor _array_element))
        (Default|Erreur _asbp_maire (Utilities|Array|MakeArray "Vous voilà désormais membre de la guilde ! 
 
Vous devez désormais accomplir vos tâches de membre ! 
 
Passons ensemble en revue les activités des apothicaires !" "Les apothicaires sont avant tout des aventuriers qui explorent le monde afin de trouver des plantes médicinales permettant de concevoir leurs solutions. 
 
On trouve de ces plantes partout, toutes ont des effets et efficacités différentes. 
 
Vous aussi, vous partirez à l'aventure pour en trouver. Pourquoi pas commencer par les plaines vertes au nord du village ?" "Lorsqu'ils n'explorent pas le monde, les apothicaires sont bien souvent en train de tester des nouvelles concoctions dans leur laboratoire.  
 
Pour cela, ils mélangent des catalyseurs stockés dans des coffres rouges et des ingrédients à effets, stockés dans les coffres marrons. 
 
Cela leur permet de créer des combinaisons infinies permettant de soigner efficacement !" "Les membres de la guilde ne sont pas utiles que pour leurs concoctions.  
Ils sont aussi très appréciés pour l'aide qu'ils apportent aux différents habitants en réglant leurs problèmes. Essaye vous-aussi de discuter avec eux. Peut-être que vous pourrez leur venir en aide !") (Utilities|Array|MakeArray "Félicitations !" "1. Aventure" "2. Concoctions" "3. Aider") (Utilities|Array|MakeArray (Utilities|Struct|MakeSlateBrush "Image" "NoTile" "NoMirror" "(X=32.000000,Y=32.000000)" "(Left=0.000000,Top=0.000000,Right=0.000000,Bottom=0.000000)" "(SpecifiedColor=(R=1.000000,G=1.000000,B=1.000000,A=1.000000),ColorUseRule=UseColor_Specified)" "(CornerRadii=(X=0.000000,Y=0.000000,Z=0.000000,W=1.000000),Color=(SpecifiedColor=(R=0.000000,G=0.000000,B=0.000000,A=0.000000),ColorUseRule=UseColor_Specified),Width=0.000000,RoundingType=HalfHeightRadius,bUseBrushTransparency=False)" "/Game/UI/Tutorials/images_tuto/TS1.TS1") (Utilities|Struct|MakeSlateBrush "Image" "NoTile" "NoMirror" "(X=32.000000,Y=32.000000)" "(Left=0.000000,Top=0.000000,Right=0.000000,Bottom=0.000000)" "(SpecifiedColor=(R=1.000000,G=1.000000,B=1.000000,A=1.000000),ColorUseRule=UseColor_Specified)" "(CornerRadii=(X=0.000000,Y=0.000000,Z=0.000000,W=1.000000),Color=(SpecifiedColor=(R=0.000000,G=0.000000,B=0.000000,A=0.000000),ColorUseRule=UseColor_Specified),Width=0.000000,RoundingType=HalfHeightRadius,bUseBrushTransparency=False)" "/Game/UI/Tutorials/images_tuto/TS2.TS2") (Utilities|Struct|MakeSlateBrush "Image" "NoTile" "NoMirror" "(X=32.000000,Y=32.000000)" "(Left=0.000000,Top=0.000000,Right=0.000000,Bottom=0.000000)" "(SpecifiedColor=(R=1.000000,G=1.000000,B=1.000000,A=1.000000),ColorUseRule=UseColor_Specified)" "(CornerRadii=(X=0.000000,Y=0.000000,Z=0.000000,W=1.000000),Color=(SpecifiedColor=(R=0.000000,G=0.000000,B=0.000000,A=0.000000),ColorUseRule=UseColor_Specified),Width=0.000000,RoundingType=HalfHeightRadius,bUseBrushTransparency=False)" "/Game/UI/Tutorials/images_tuto/TS3.TS3") (Utilities|Struct|MakeSlateBrush "Image" "NoTile" "NoMirror" "(X=32.000000,Y=32.000000)" "(Left=0.000000,Top=0.000000,Right=0.000000,Bottom=0.000000)" "(SpecifiedColor=(R=1.000000,G=1.000000,B=1.000000,A=1.000000),ColorUseRule=UseColor_Specified)" "(CornerRadii=(X=0.000000,Y=0.000000,Z=0.000000,W=1.000000),Color=(SpecifiedColor=(R=0.000000,G=0.000000,B=0.000000,A=0.000000),ColorUseRule=UseColor_Specified),Width=0.000000,RoundingType=HalfHeightRadius,bUseBrushTransparency=False)" "/Game/UI/Tutorials/images_tuto/TS4.TS4")))))))

(event EventBeginPlay
  (|CallParentFunction) ; This node is disabled and will not be called.\nDrag off pins to build functionality.
)

(event Collision|EventActorBeginOverlap
  (params (OtherActor :type Actor%20Object%20Reference))
  (|CallParentFunction OtherActor) ; This node is disabled and will not be called.\nDrag off pins to build functionality.
)

(event EventTick
  (params (DeltaSeconds :type Float%20%28single-precision%29))
  (|CallParentFunction DeltaSeconds) ; This node is disabled and will not be called.\nDrag off pins to build functionality.
)

(fn ConstructionScript
  (|CallParentFunction))