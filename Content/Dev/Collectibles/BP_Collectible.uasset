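; BP_Collectible is a pickup actor that adds an ingredient to the player's collection.
; On BeginPlay it caches the third-person character, sets its cube's material by rarity and copies its name to EntryText.
; A one-time Interaction event shows a WB_Item widget, constructs a BP_Ingredient object from its properties with the character as outer, appends it to the character's Ingredients array and destroys the actor.
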(event EventBeginPlay
  (|CallParentFunction)
  (bind _asbp_third_person_character (Utilities|Casting|CastToBP_ThirdPersonCharacter (Game|GetPlayerCharacter 0)))
  (Variables|Default|SetAs%20BP%20Third%20Person%20Character _asbp_third_person_character)
  (CallFunction|SetMaterial)
  (Variables|Default|SetEntry_text (Variables|Default|GetName)))

(event Collision|EventActorBeginOverlap
  (params (OtherActor :type Actor%20Object%20Reference))
  (|CallParentFunction OtherActor) ; This node is disabled and will not be called.\nDrag off pins to build functionality.
)

(event EventTick
  (params (DeltaSeconds :type Float%20%28single-precision%29))
  (|CallParentFunction DeltaSeconds) ; This node is disabled and will not be called.\nDrag off pins to build functionality.
)

(event EventInteraction
  (bind _as_bp_third_person_character (Variables|Default|GetAs%20BP%20Third%20Person%20Character))
  (Utilities|FlowControl|DoOnce false
    (:Completed
      (bind _returnvalue (UserInterface|CreateWidget "/Game/UI/Character/WB_Item.WB_Item_C" 0 (Variables|Default|GetBrush) (Utilities|Text|ToText(String) (Variables|Default|GetName))))
      (UserInterface|Viewport|AddtoViewport _returnvalue 0)
      (bind _returnvalue_2 (Game|ConstructObjectfromClass _as_bp_third_person_character "/Game/Dev/Collectibles/BP_Ingredient.BP_Ingredient_C" (Variables|Default|GetName) (Variables|Default|GetInstance_Name) (Variables|Default|GetEfficiency) (Variables|Default|GetRarity) (Variables|Default|GetIs_Catalyst) (Variables|Default|GetCatalyst_type) (Variables|Default|GetBrush)))
      (Utilities|Array|Add (Variables|/Game/ThirdPerson/Blueprints/BP_ThirdPersonCharacter.BP_ThirdPersonCharacter_C|GetIngredients _as_bp_third_person_character) _returnvalue_2)
      (Development|PrintString (Variables|Default|GetName))
      (Actor|DestroyActor))))

(fn ConstructionScript
  (|CallParentFunction))

(fn SetMaterial
  (switch Utilities|FlowControl|Switch|SwitchonEnum_Rarity (Variables|Default|GetRarity)
    (:NewEnumerator0
      (LocalVariables|SetMaterial "/Game/Dev/Materials/M_Basic.M_Basic"))
    (:NewEnumerator1
      (LocalVariables|SetMaterial "/Game/Dev/Materials/M_Rare.M_Rare"))
    (:NewEnumerator2
      (LocalVariables|SetMaterial "/Game/Dev/Materials/M_Epic.M_Epic"))
    (:NewEnumerator3
      (LocalVariables|SetMaterial "/Game/Dev/Materials/M_Legendary.M_Legendary")))
  (Rendering|Material|SetMaterial (Variables|Default|GetCube) 0 (LocalVariables|GetMaterial)))