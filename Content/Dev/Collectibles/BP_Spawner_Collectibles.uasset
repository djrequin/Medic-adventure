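; Spawner actor that places one random BP_Collectible at its location on BeginPlay.
; It rolls an item rarity weighted by its spawner tier, with higher tiers able to yield nothing.
; It then shuffles DT_Collectibles rows matching that rarity and the spawner's localization, and spawns the first with randomized efficiency.
; A respawn event bound through BP_ThirdPersonGameMode destroys the current collectible and rerolls.
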(event Custom|New_Spawn
  (Utilities|IsValid (Variables|Default|GetSpawned_Collectible)
    (:Is%20Valid
      (Actor|DestroyActor (Variables|Default|GetSpawned_Collectible))
      (Variables|Default|SetSpawned_Collectible 0))
    (:Is%20Not%20Valid
      _))
  (CallFunction|SpawnItem))

(event EventBeginPlay
  (|CallParentFunction)
  (CallFunction|SpawnItem)
  (bind _asbp_third_person_game_mode (Utilities|Casting|CastToBP_ThirdPersonGameMode (Game|GetGameMode)))
  (EventDispatchers|BindEventtoRespawnItems _asbp_third_person_game_mode (delegate Custom|New_Spawn)))

(event Collision|EventActorBeginOverlap
  (params (OtherActor :type Actor%20Object%20Reference))
  (|CallParentFunction OtherActor) ; This node is disabled and will not be called.\nDrag off pins to build functionality.
)

(event EventTick
  (params (DeltaSeconds :type Float%20%28single-precision%29))
  (|CallParentFunction DeltaSeconds) ; This node is disabled and will not be called.\nDrag off pins to build functionality.
)

(fn ConstructionScript
  (|CallParentFunction))

(fn DefineCollectible
  (bind _choosed_item (LocalVariables|GetChoosed_item))
  ;[1 1 1] Obtention des données
  (bind _outrownames (DataTable|GetDataTableRowNames "/Game/Dev/Collectibles/DT_Collectibles.DT_Collectibles"))
  (for _array_element _outrownames
    (bind _returnvalue (Utilities|GetDataTableRow "/Game/Dev/Collectibles/DT_Collectibles.DT_Collectibles" _array_element)
      (:then
        ;[1 1 1] Bonne localisation ?
        (for _array_element_2 (.Item_localisation (Utilities|Struct|BreakStruct_Collect _returnvalue))
          (if (and (Utilities|Enum|Equal(Enum) _array_element_2 (Variables|Default|GetSpawner_Localization)) (Utilities|Enum|Equal(Enum) (.Rarity (Utilities|Struct|BreakStruct_Collect _returnvalue)) (Variables|Default|GetItem_rarity)))
            ;[1 1 1] Liste des items correspondants
            (Utilities|Array|Add (LocalVariables|GetChoosed_item) _returnvalue)
            (LocalVariables|SetFound%20? true))))))
  ;[1 1 1] Mélange du tableau
  (Utilities|Array|Shuffle _choosed_item)
  (return (Utilities|Array|Get(acopy) _choosed_item) (LocalVariables|GetFound%20?)))

(fn DefineItemRarity
  ;[1 1 1] Check de la rareté voulue
  (switch Utilities|FlowControl|Switch|SwitchonEnum_Rarity (Variables|Default|GetSpawner_Rarity)
    (:NewEnumerator0
      ;[1 1 1] Calcul des différentes proba
      (bind (_chosen_rarity _can_spawn) (Rarity_selectors|BasicRarity))
      (Variables|Default|SetItem_rarity _chosen_rarity)
      (LocalVariables|SetSpawn? _can_spawn))
    (:NewEnumerator1
      (bind (_chosen_rarity_2 _spawn_) (Rarity_selectors|RareRarity))
      (Variables|Default|SetItem_rarity _chosen_rarity_2)
      (LocalVariables|SetSpawn? _spawn_))
    (:NewEnumerator2
      (bind (_chosen_rarity_3 _spawn__2) (Rarity_selectors|EpicRarity))
      (Variables|Default|SetItem_rarity _chosen_rarity_3)
      (LocalVariables|SetSpawn? _spawn__2))
    (:NewEnumerator3
      (bind (_chosen_rarity_4 _spawn__3) (Rarity_selectors|LegendaryRarity))
      (Variables|Default|SetItem_rarity _chosen_rarity_4)
      (LocalVariables|SetSpawn? _spawn__3)))
  (return (LocalVariables|GetSpawn?)))

(fn BasicRarity
  (if (<= (Math|Random|RandomIntegerinRange 1 100) 75)
    (LocalVariables|SetLocal_Rarity "NewEnumerator0")
    (else
      (LocalVariables|SetLocal_Rarity "NewEnumerator1")))
  (return (LocalVariables|GetLocal_Rarity) true))

(fn RareRarity
  (LocalVariables|SetNumber (Math|Random|RandomIntegerinRange 1 100))
  (if (Math|Integer|InRange(Integer) (LocalVariables|GetNumber) 0 20)
    (LocalVariables|SetLocal_Rarity "NewEnumerator0")
    (elif (Math|Integer|InRange(Integer) (LocalVariables|GetNumber) 20 75)
      (LocalVariables|SetLocal_Rarity "NewEnumerator1")
      (elif (Math|Integer|InRange(Integer) (LocalVariables|GetNumber) 75 90)
        (LocalVariables|SetLocal_Rarity "NewEnumerator2")
        (else
          (LocalVariables|SetCan_Spawn false)))))
  (return (LocalVariables|GetLocal_Rarity) (LocalVariables|GetCan_Spawn)))

(fn EpicRarity
  (LocalVariables|SetNumber (Math|Random|RandomIntegerinRange 1 100))
  (if (Math|Integer|InRange(Integer) (LocalVariables|GetNumber) 0 20)
    (LocalVariables|SetLocal_Rarity "NewEnumerator1")
    (elif (Math|Integer|InRange(Integer) (LocalVariables|GetNumber) 20 80)
      (LocalVariables|SetLocal_Rarity "NewEnumerator2")
      (elif (Math|Integer|InRange(Integer) (LocalVariables|GetNumber) 80 90)
        (LocalVariables|SetLocal_Rarity "NewEnumerator3")
        (else
          (LocalVariables|SetCan_Spawn false)))))
  (return (LocalVariables|GetLocal_Rarity) (LocalVariables|GetCan_Spawn)))

(fn LegendaryRarity
  (LocalVariables|SetNumber (Math|Random|RandomIntegerinRange 1 100))
  (if (Math|Integer|InRange(Integer) (LocalVariables|GetNumber) 0 15)
    (LocalVariables|SetLocal_Rarity "NewEnumerator2")
    (elif (Math|Integer|InRange(Integer) (LocalVariables|GetNumber) 15 50)
      (LocalVariables|SetLocal_Rarity "NewEnumerator3")
      (else
        (LocalVariables|SetCan_Spawn false))))
  (return (LocalVariables|GetLocal_Rarity) (LocalVariables|GetCan_Spawn)))

(fn SpawnItem
  ;[1 1 1] Définition de la rareté
  (bind _can_spawn_ (CallFunction|DefineItemRarity))
  (if _can_spawn_
    ;[1 1 1] Séléction de l'objet
    (bind (_chosen_item _found_) (CallFunction|DefineCollectible))
    (if _found_
      ;[0.8333 0.5632 0] Création de l'objet
      (bind _returnvalue (Game|SpawnActorfromClass "/Game/Dev/Collectibles/BP_Collectible.BP_Collectible_C" (Math|Transform|MakeTransform (Transformation|GetActorLocation) "0, 0, 0" "1.000000,1.000000,1.000000") "Undefined" "MultiplyWithRoot" 0 (Math|Random|RandomIntegerinRange (.min_efficiency _chosen_item) (.maxefficiency _chosen_item)) (.rarity _chosen_item) (.iscatalyst _chosen_item) (.catalysttype _chosen_item) (.instance_name _chosen_item) (.object_name _chosen_item) (.sm _chosen_item) (.ui_brush _chosen_item) (.effectivedisease _chosen_item) 0))
      (Variables|Default|SetSpawned_Collectible _returnvalue)
      (else
        (Development|PrintString "Nothing to spawn" true true "(R=1.000000,G=0.619305,B=0.000000,A=1.000000)")))
    (else
      (Development|PrintString (Utilities|String|Append "Couldn't spawn " " 
" "Selected rarity :  " (Utilities|String|EnumtoString (Variables|Default|GetSpawner_Rarity))) true true "(R=1.000000,G=0.007234,B=0.000000,A=1.000000)" 4.0))))