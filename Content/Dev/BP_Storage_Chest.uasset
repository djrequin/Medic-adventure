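; Storage chest for one ingredient type, showing that type's icon on its widget and a French "Prendre" prompt.
; When looked at, a DoOnce-gated detection flow queries the player character's sorted ingredients of that type.
; Depending on the IsEmpty result, it opens a short storage widget registered with the game mode or sets the prompt to "Vide".
; Interaction is empty, and the full storage screen logic is disconnected.
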(event EventBeginPlay
  (|CallParentFunction)
  (bind _aswb_chest_icons (Utilities|Casting|CastToWB_Chest_icons (UserInterface|GetWidget (Variables|Default|GetWidget))))
  (Default|SetImage _aswb_chest_icons (Variables|Default|GetIngredient))
  (Variables|Default|SetEntry_text (Utilities|String|Append "Prendre 
" (Utilities|String|EnumtoString (Variables|Default|GetIngredient))))
  (bind _asbp_third_person_character (Utilities|Casting|CastToBP_ThirdPersonCharacter (Game|GetPlayerCharacter 0)))
  (Variables|Default|SetAs%20BP%20Third%20Person%20Character _asbp_third_person_character)
  (bind _asbp_third_person_game_mode (Utilities|Casting|CastToBP_ThirdPersonGameMode (Game|GetGameMode)))
  (Variables|Default|SetAs%20BP%20Third%20Person%20Game%20Mode _asbp_third_person_game_mode))

(event Collision|EventActorBeginOverlap
  (params (OtherActor :type Actor%20Object%20Reference))
  (|CallParentFunction OtherActor) ; This node is disabled and will not be called.\nDrag off pins to build functionality.
)

(event EventTick
  (params (DeltaSeconds :type Float%20%28single-precision%29))
  (|CallParentFunction DeltaSeconds) ; This node is disabled and will not be called.\nDrag off pins to build functionality.
)

(event EventInteraction)

(event EventPostDetection
  (bind _as_bp_third_person_character (Variables|Default|GetAs%20BP%20Third%20Person%20Character))
  (bind _ingredient (Variables|Default|GetIngredient))
  (bind (_correponding_ingredients _is_empty_) (Default|SortIngredients _as_bp_third_person_character _ingredient))
  (Default|RemoveWidget (Variables|Default|GetAs%20BP%20Third%20Person%20Game%20Mode))
  (Utilities|FlowControl|DoOnce false) ; enters at Reset
)

(event EventLookingEvent
  (bind _as_bp_third_person_character (Variables|Default|GetAs%20BP%20Third%20Person%20Character))
  (bind _ingredient (Variables|Default|GetIngredient))
  (bind (_correponding_ingredients _is_empty_) (Default|SortIngredients _as_bp_third_person_character _ingredient))
  (Utilities|FlowControl|DoOnce false
    (:Completed
      (if _is_empty_
        (Variables|Default|SetShow? true)
        (Default|RemoveWidget (Variables|Default|GetAs%20BP%20Third%20Person%20Game%20Mode))
        (Variables|Default|SetEntry_text (Utilities|String|Append))
        (bind _returnvalue (UserInterface|CreateWidget "/Game/UI/Character/WB_Short_storage.WB_Short_storage_C" 0 _correponding_ingredients (Variables|Default|Getcatalyst?) (Variables|Default|GetDescription)))
        (Utilities|Array|Add (Variables|/Game/ThirdPerson/Blueprints/BP_ThirdPersonGameMode.BP_ThirdPersonGameMode_C|GetOpened_storage (Variables|Default|GetAs%20BP%20Third%20Person%20Game%20Mode)) _returnvalue)
        (UserInterface|Viewport|AddtoViewport _returnvalue 0)
        (Development|PrintString "looking")
        (else
          (Default|RemoveWidget (Variables|Default|GetAs%20BP%20Third%20Person%20Game%20Mode))
          (Variables|Default|SetEntry_text "Vide"))))))

(fn ConstructionScript
  (|CallParentFunction))

(fn Init)