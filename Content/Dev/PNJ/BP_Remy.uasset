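; BP_Remy is an NPC whose dialogue choice asks the player for 1000 gold to save a woman.
; When the choice appears it shows a money widget; the upper choice runs a money check, the bottom choice makes Remy urge haste.
; A successful check deducts the gold and clears PostDialogChoice, while a failed one opens a complaint quoting the player's current balance.
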(event EventBeginPlay
  (|CallParentFunction) ; This node is disabled and will not be called.\nDrag off pins to build functionality.
)

(event Collision|EventActorBeginOverlap
  (params (OtherActor :type Actor%20Object%20Reference))
  (|CallParentFunction OtherActor) ; This node is disabled and will not be called.\nDrag off pins to build functionality.
)

(event EventTick
  (params (DeltaSeconds :type Float%20%28single-precision%29))
  (|CallParentFunction DeltaSeconds) ; This node is disabled and will not be called.\nDrag off pins to build functionality.
)

(event EventUpperChoice
  (params (Widget :type WB%20Dialog%20System%20Object%20Reference))
  (CallFunction|CheckPlayerMoney Widget))

(event EventBottomChoice
  (params (Widget :type WB%20Dialog%20System%20Object%20Reference))
  (Widget|RemovefromParent Widget)
  (bind _returnvalue (UserInterface|CreateWidget "/Game/UI/Story/WB_Dialog_system.WB_Dialog_system_C" 0 (Utilities|Array|MakeArray (Variables|Default|GetChara_name)) (Utilities|Array|MakeArray "Dépêche toi, elle a vraiment besoin d'aide.") false 0))
  (UserInterface|Viewport|AddtoViewport _returnvalue 0)
  (Widget|RemovefromParent (Variables|Default|Getwidget)))

(event EventChoiceAppaearEvent
  (bind _returnvalue (UserInterface|CreateWidget "/Game/UI/WB_Money_Changes.WB_Money_Changes_C"))
  (Variables|Default|Setwidget _returnvalue)
  (UserInterface|Viewport|AddtoViewport _returnvalue 0))

(fn ConstructionScript
  (|CallParentFunction))

(fn CheckPlayerMoney
  (params (NewParam :type WB%20Dialog%20System%20Object%20Reference))
  (bind _as_bp_third_person_character (Variables|Default|GetAs%20BP%20Third%20Person%20Character))
  (if (>= (Variables|/Game/ThirdPerson/Blueprints/BP_ThirdPersonCharacter.BP_ThirdPersonCharacter_C|GetMoney _as_bp_third_person_character) 1000)
    (Variables|/Game/ThirdPerson/Blueprints/BP_ThirdPersonCharacter.BP_ThirdPersonCharacter_C|SetMoney _as_bp_third_person_character (- (Variables|/Game/ThirdPerson/Blueprints/BP_ThirdPersonCharacter.BP_ThirdPersonCharacter_C|GetMoney _as_bp_third_person_character) 1000))
    (Widget|RemovefromParent NewParam)
    (bind _returnvalue (UserInterface|CreateWidget "/Game/UI/Story/WB_Dialog_system.WB_Dialog_system_C" 0 (Utilities|Array|MakeArray (Variables|Default|GetChara_name)) (Utilities|Array|MakeArray "Hehehehe.") false self))
    (UserInterface|Viewport|AddtoViewport _returnvalue 0)
    (Variables|Default|SetPost_dialog_choice? false)
    (else
      (Widget|RemovefromParent NewParam)
      (bind _returnvalue_2 (UserInterface|CreateWidget "/Game/UI/Story/WB_Dialog_system.WB_Dialog_system_C" 0 (Utilities|Array|MakeArray (Variables|Default|GetChara_name)) (Utilities|Array|MakeArray (Utilities|String|Append "Mais... C'est carrément pas assez. Comment tu veux que je la sauve avec seulement " (Utilities|String|ToString(Integer) (Variables|/Game/ThirdPerson/Blueprints/BP_ThirdPersonCharacter.BP_ThirdPersonCharacter_C|GetMoney (.AsBP%20Third%20Person%20Character (Utilities|Casting|CastToBP_ThirdPersonCharacter (Game|GetPlayerCharacter 0))))) " pièces d'or !?")) false self))
      (UserInterface|Viewport|AddtoViewport _returnvalue_2 0)
      (Widget|RemovefromParent (Variables|Default|Getwidget)))))