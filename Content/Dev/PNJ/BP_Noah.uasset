(event EventBeginPlay
  (|CallParentFunction))

(event Collision|EventActorBeginOverlap
  (params (OtherActor :type Actor%20Object%20Reference))
  (|CallParentFunction OtherActor) ; This node is disabled and will not be called.\nDrag off pins to build functionality.
)

(event EventTick
  (params (DeltaSeconds :type Float%20%28single-precision%29))
  (|CallParentFunction DeltaSeconds) ; This node is disabled and will not be called.\nDrag off pins to build functionality.
)

(event EventPostDialogEvent
  (Development|PrintString "JB post dialog"))

(event EventUpperChoice
  (params (Widget :type WB%20Dialog%20System%20Object%20Reference))
  (Development|PrintString "C'était upper")
  (CallFunction|CheckPlayerMoney Widget))

(event EventBottomChoice
  (params (Widget :type WB%20Dialog%20System%20Object%20Reference))
  (Development|PrintString "C'était bottom")
  (Variables|Default|SetPost_dialog_choice? false))

(fn ConstructionScript
  (|CallParentFunction))

(fn CheckPlayerMoney
  (params (NewParam :type WB%20Dialog%20System%20Object%20Reference))
  (bind _as_bp_third_person_character (Variables|Default|GetAs%20BP%20Third%20Person%20Character))
  (if (>= (Variables|/Game/ThirdPerson/Blueprints/BP_ThirdPersonCharacter.BP_ThirdPersonCharacter_C|GetMoney _as_bp_third_person_character) 6)
    (Variables|/Game/ThirdPerson/Blueprints/BP_ThirdPersonCharacter.BP_ThirdPersonCharacter_C|SetMoney _as_bp_third_person_character (- (Variables|/Game/ThirdPerson/Blueprints/BP_ThirdPersonCharacter.BP_ThirdPersonCharacter_C|GetMoney _as_bp_third_person_character) 6))
    (Widget|RemovefromParent NewParam)
    (bind _returnvalue (UserInterface|CreateWidget "/Game/UI/Story/WB_Dialog_system.WB_Dialog_system_C" 0 (Utilities|Array|MakeArray "Jean-Baptiste") (Utilities|Array|MakeArray "Merci pour ton aide !") false self))
    (UserInterface|Viewport|AddtoViewport _returnvalue 0)
    (Variables|Default|SetPost_dialog_choice? false)
    (else
      (Widget|RemovefromParent NewParam)
      (bind _returnvalue_2 (UserInterface|CreateWidget "/Game/UI/Story/WB_Dialog_system.WB_Dialog_system_C" 0 (Utilities|Array|MakeArray "Jean-Baptiste") (Utilities|Array|MakeArray "T'as pas assez non plus...") false self))
      (UserInterface|Viewport|AddtoViewport _returnvalue_2 0))))