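; BP_ND is a dialog trigger actor that opens WB_Dialog_system with its ANames and AContents and disables player character input.
; The Overlap flag picks the trigger: Interaction opens the dialog when it is off, and entering the Box as BP_ThirdPersonCharacter opens it when on.
; Overlap mode sets Show to false at BeginPlay and uses a DoOnce that resets when the character leaves the Box.
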(event OnComponentBeginOverlap(Box)
  (params (OverlappedComponent :type Primitive%20Component%20Object%20Reference) (OtherActor :type Actor%20Object%20Reference) (OtherComp :type Primitive%20Component%20Object%20Reference) (OtherBodyIndex :type Integer) (bFromSweep :type Boolean) (SweepResult :type Hit%20Result%20Structure%20%28by%20ref%29))
  (Utilities|Casting|CastToBP_ThirdPersonCharacter OtherActor)
  (if (Variables|Default|GetOverlap%20?)
    (Utilities|FlowControl|DoOnce false
      (:Completed
        (Input|DisableInput (Game|GetPlayerCharacter 0) (Game|GetPlayerController 0))
        (bind _returnvalue (UserInterface|CreateWidget "/Game/UI/Story/WB_Dialog_system.WB_Dialog_system_C" 0 (Variables|Default|GetA%20Names) (Variables|Default|GetA%20Contents) false 0))
        (UserInterface|Viewport|AddtoViewport _returnvalue 0)))))

(event OnComponentEndOverlap(Box)
  (params (OverlappedComponent :type Primitive%20Component%20Object%20Reference) (OtherActor :type Actor%20Object%20Reference) (OtherComp :type Primitive%20Component%20Object%20Reference) (OtherBodyIndex :type Integer))
  (Utilities|Casting|CastToBP_ThirdPersonCharacter OtherActor)
  (Utilities|FlowControl|DoOnce false) ; enters at Reset
)

(event EventBeginPlay
  (|CallParentFunction)
  (if (Variables|Default|GetOverlap%20?)
    (Variables|Default|SetShow? false)))

(event Collision|EventActorBeginOverlap
  (params (OtherActor :type Actor%20Object%20Reference))
  (|CallParentFunction OtherActor) ; This node is disabled and will not be called.\nDrag off pins to build functionality.
)

(event EventTick
  (params (DeltaSeconds :type Float%20%28single-precision%29))
  (|CallParentFunction DeltaSeconds) ; This node is disabled and will not be called.\nDrag off pins to build functionality.
)

(event EventInteraction
  (if (not (Variables|Default|GetOverlap%20?))
    (Input|DisableInput (Game|GetPlayerCharacter 0) (Game|GetPlayerController 0))
    (bind _returnvalue (UserInterface|CreateWidget "/Game/UI/Story/WB_Dialog_system.WB_Dialog_system_C" 0 (Variables|Default|GetA%20Names) (Variables|Default|GetA%20Contents) false 0))
    (UserInterface|Viewport|AddtoViewport _returnvalue 0)))

(fn ConstructionScript
  (|CallParentFunction))