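; BP_Eymira is an NPC who offers the player a ride back, teleporting them to a spawn point.
; Upper and bottom choice events close the choice widget and open an accept or decline dialog.
; Only the accept dialog receives this NPC as its PNJ reference, though both set the post-dialog flag.
; PostDialogEvent shows a black transition, waits briefly, then sets the player capsule's location and rotation to the SpawnPoint's.
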(event EventBeginPlay
  (|CallParentFunction) ; This node is disabled and will not be called.\nDrag off pins to build functionality.
)

(event Collision|EventActorBeginOverlap
  (params (OtherActor :type Actor%20Object%20Reference))
  (|CallParentFunction OtherActor) ; This node is disabled and will not be called.\nDrag off pins to build functionality.
)

(event EventTick
  (params (DeltaSeconds :type Float%20%28single-precision%29))
  (|CallParentFunction DeltaSeconds) ; This node is disabled and will not be called.\nDrag off pins to build functionality.
)

(event EventUpperChoice
  (params (Widget :type WB%20Dialog%20System%20Object%20Reference))
  (Widget|RemovefromParent Widget)
  (bind _returnvalue (UserInterface|CreateWidget "/Game/UI/Story/WB_Dialog_system.WB_Dialog_system_C" 0 (Utilities|Array|MakeArray (Variables|Default|GetChara_name)) (Utilities|Array|MakeArray "Ok, c'est parti, accroche toi bien !") false self false true))
  (UserInterface|Viewport|AddtoViewport _returnvalue 0))

(event EventBottomChoice
  (params (Widget :type WB%20Dialog%20System%20Object%20Reference))
  (Widget|RemovefromParent Widget)
  (bind _returnvalue (UserInterface|CreateWidget "/Game/UI/Story/WB_Dialog_system.WB_Dialog_system_C" 0 (Utilities|Array|MakeArray (Variables|Default|GetChara_name)) (Utilities|Array|MakeArray "Pas de problèmes, n'hésite pas à venir me voir si tu veux rentrer !") false 0 false true))
  (UserInterface|Viewport|AddtoViewport _returnvalue 0))

(event EventPostDialogEvent
  (bind _returnvalue (Game|GetPlayerCharacter 0))
  (bind _spawn_point (Variables|Default|GetSpawn_point))
  (bind _capsulecomponent (Variables|/Script/Engine.Character|GetCapsuleComponent _returnvalue))
  (bind _returnvalue_2 (UserInterface|CreateWidget "/Game/UI/WB_Transi_Black.WB_Transi_Black_C"))
  (UserInterface|Viewport|AddtoViewport _returnvalue_2 0)
  (Utilities|FlowControl|Delay 1.2)
  (Transformation|SetWorldLocation _capsulecomponent (Transformation|GetActorLocation _spawn_point) false false)
  (Transformation|SetWorldRotation _capsulecomponent (Transformation|GetActorRotation _spawn_point) false false))

(fn ConstructionScript
  (|CallParentFunction))