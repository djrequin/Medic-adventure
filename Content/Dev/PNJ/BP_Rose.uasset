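; Rose is a quest NPC, a child of a dialog NPC class, who needs the "Onguent Grobobo" ointment to return to the guild.
; After her first dialog she gives the player a Baies ingredient and enables a choice prompt.
; Accepting consumes the ointment if owned and clears Switch, so the next post-dialog event fades to black, relocates her to TP, resets her dialog and destroys BV.
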(event EventBeginPlay
  (|CallParentFunction) ; This node is disabled and will not be called.\nDrag off pins to build functionality.
)

(event Collision|EventActorBeginOverlap
  (params (OtherActor :type Actor%20Object%20Reference))
  (|CallParentFunction OtherActor) ; This node is disabled and will not be called.\nDrag off pins to build functionality.
)

(event EventTick
  (params (DeltaSeconds :type Float%20%28single-precision%29))
  (|CallParentFunction DeltaSeconds) ; This node is disabled and will not be called.\nDrag off pins to build functionality.
)

(event EventUpperChoice
  (params (Widget :type WB%20Dialog%20System%20Object%20Reference))
  (bind _chara_name (Variables|Default|GetChara_name))
  (Widget|RemovefromParent Widget)
  (bind _found_ (CallFunction|SearchMedoc))
  (if _found_
    (bind _returnvalue (UserInterface|CreateWidget "/Game/UI/Story/WB_Dialog_system.WB_Dialog_system_C" 0 (Utilities|Array|MakeArray _chara_name _chara_name _chara_name) (Utilities|Array|MakeArray "Oh tu m'en a rapporté un ! " "Merci beaucoup, grâce à toi, je vais pouvoir rentrer à la guilde." "On se reverra là-bas !") false self false true))
    (UserInterface|Viewport|AddtoViewport _returnvalue 0)
    (Variables|Default|SetSwitch false)
    (else
      (bind _returnvalue_2 (UserInterface|CreateWidget "/Game/UI/Story/WB_Dialog_system.WB_Dialog_system_C" 0 (Utilities|Array|MakeArray (Variables|Default|GetChara_name)) (Utilities|Array|MakeArray "Je suis désolée, mais tu n'as aucun onguent adapté...") false self))
      (UserInterface|Viewport|AddtoViewport _returnvalue_2 0))))

(event EventBottomChoice
  (params (Widget :type WB%20Dialog%20System%20Object%20Reference))
  (Widget|RemovefromParent Widget)
  (bind _returnvalue (UserInterface|CreateWidget "/Game/UI/Story/WB_Dialog_system.WB_Dialog_system_C" 0 (Utilities|Array|MakeArray (Variables|Default|GetChara_name)) (Utilities|Array|MakeArray "Je comprends, mais reviens vite s'il te plaît.") false self))
  (UserInterface|Viewport|AddtoViewport _returnvalue 0))

(event EventPostDialogEvent
  (bind _returnvalue (Game|GetPlayerCharacter 0))
  (bind _brush (Variables|Default|GetBrush))
  (bind _capsulecomponent (Variables|Default|GetCapsuleComponent))
  (bind _tp (Variables|Default|GetTP))
  (bind _asbp_third_person_character (Utilities|Casting|CastToBP_ThirdPersonCharacter _returnvalue))
  (if (Variables|Default|GetSwitch)
    (Variables|Default|SetPost_dialog_event? false)
    (Variables|Default|SetPost_dialog_choice? true)
    (bind _returnvalue_2 (Game|ConstructObjectfromClass "/Game/Dev/Collectibles/BP_Ingredient.BP_Ingredient_C" "Baies" "NewEnumerator7" 7 "NewEnumerator2" true "NewEnumerator0" _brush "NewEnumerator0" "Baies"))
    (Utilities|Array|Add (Variables|/Game/ThirdPerson/Blueprints/BP_ThirdPersonCharacter.BP_ThirdPersonCharacter_C|GetIngredients _asbp_third_person_character) _returnvalue_2)
    (bind _returnvalue_3 (UserInterface|CreateWidget "/Game/UI/Character/WB_Item.WB_Item_C" 0 _brush "Baies" (.Possessed (Default|CountIngredients _asbp_third_person_character "NewEnumerator7"))))
    (UserInterface|Viewport|AddtoViewport _returnvalue_3 0)
    (Utilities|Array|RemoveItem (Variables|Default|GetContents) (Utilities|Array|Get(acopy) (Variables|Default|GetContents) (Utilities|Array|LastIndex (Variables|Default|GetContents))))
    (else
      (bind _returnvalue_4 (UserInterface|CreateWidget "/Game/UI/WB_Transi_Black.WB_Transi_Black_C"))
      (UserInterface|Viewport|AddtoViewport _returnvalue_4 0)
      (Utilities|FlowControl|Delay 1.2)
      (Transformation|SetWorldLocation _capsulecomponent (Transformation|GetActorLocation _tp) false false)
      (Transformation|SetWorldRotation _capsulecomponent (Transformation|GetActorRotation _tp) false false)
      (Utilities|FlowControl|Sequence
        (:then_0
          (Variables|Default|SetContents (Utilities|Array|MakeArray "Oh tu es celui qui m'a aidée l'autre jour." "J'espère que tes aventures se passent bien. Si un jour tu es en difficulté, viens me voir !"))
          (Variables|Default|SetCanBeSick true)
          (Variables|Default|SetPost_dialog_choice? false))
        (:then_1
          (Variables|Default|SetNames (Utilities|Array|MakeArray "NewEnumerator16" "NewEnumerator16")))
        (:then_2
          (CallFunction|ConvertNames))
        (:then_3
          (Actor|DestroyActor (Variables|Default|GetBV)))))))

(fn ConstructionScript
  (|CallParentFunction))

(fn SearchMedoc
  (bind _as_bp_third_person_character (Variables|Default|GetAs%20BP%20Third%20Person%20Character))
  (bind _medocs (Variables|/Game/ThirdPerson/Blueprints/BP_ThirdPersonCharacter.BP_ThirdPersonCharacter_C|GetMedocs _as_bp_third_person_character))
  (bind _array_element (Utilities|Array|ForEachLoopwithBreak _medocs :!label _label)
    (:LoopBody
      (if (Utilities|Enum|Equal(Enum) (Variables|/Game/ThirdPerson/Blueprints/BP_Medicament.BP_Medicament_C|GetName _array_element) "Onguent Grobobo")
        (Utilities|Array|RemoveItem _medocs _array_element)
        (LocalVariables|SetFound true)
        (goto _label Break)))
    (:Completed
      (return (LocalVariables|GetFound)))))