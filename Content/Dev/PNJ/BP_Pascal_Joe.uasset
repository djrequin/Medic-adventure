(event EventBeginPlay
  (|CallParentFunction) ; This node is disabled and will not be called.\nDrag off pins to build functionality.
)

(event Collision|EventActorBeginOverlap
  (params (OtherActor :type Actor%20Object%20Reference))
  (|CallParentFunction OtherActor) ; This node is disabled and will not be called.\nDrag off pins to build functionality.
)

(event EventTick
  (params (DeltaSeconds :type Float%20%28single-precision%29))
  (|CallParentFunction DeltaSeconds) ; This node is disabled and will not be called.\nDrag off pins to build functionality.
)

(event EventBottomChoice
  (params (Widget :type WB%20Dialog%20System%20Object%20Reference))
  (Widget|RemovefromParent Widget)
  (bind _returnvalue (UserInterface|CreateWidget "/Game/UI/Story/WB_Dialog_system.WB_Dialog_system_C" 0 (Utilities|Array|MakeArray "Pascal Joe") (Utilities|Array|MakeArray "Si tu n'as rien pour moi, ne me fais pas perdre mon temps.") false self))
  (UserInterface|Viewport|AddtoViewport _returnvalue 0))

(event EventUpperChoice
  (params (Widget :type WB%20Dialog%20System%20Object%20Reference))
  (bind _found__ (CallFunction|CheckCoquillage))
  (if _found__
    (Widget|RemovefromParent Widget)
    (bind _returnvalue (UserInterface|CreateWidget "/Game/UI/Story/WB_Dialog_system.WB_Dialog_system_C" 0 (Utilities|Array|MakeArray "Pascal Joe") (Utilities|Array|MakeArray "Oh tu me le donnes ? Merci beaucoup, tiens, voici ta récompense.") false self))
    (UserInterface|Viewport|AddtoViewport _returnvalue 0)
    (Variables|Default|SetPost_dialog_choice? false)
    (Utilities|FlowControl|Sequence
      (:then_0
        (Variables|Default|SetContents (Utilities|Array|MakeArray "Merci de m'avoir aidé mon petit" "Grâce à toi, j'aurais un beau champ." "Reviens quand tu veux !")))
      (:then_1
        (Variables|Default|SetNames (Utilities|Array|MakeArray "NewEnumerator4" "NewEnumerator4" "NewEnumerator4")))
      (:then_2
        (CallFunction|ConvertNames)))
    (else
      (Widget|RemovefromParent Widget)
      (bind _returnvalue_2 (UserInterface|CreateWidget "/Game/UI/Story/WB_Dialog_system.WB_Dialog_system_C" 0 (Utilities|Array|MakeArray "Pascal Joe") (Utilities|Array|MakeArray "Si tu n'as rien pour moi, ne me fais pas perdre mon temps.") false self))
      (UserInterface|Viewport|AddtoViewport _returnvalue_2 0))))

(fn ConstructionScript
  (|CallParentFunction))

(fn CheckCoquillage
  (bind _as_bp_third_person_character (Variables|Default|GetAs%20BP%20Third%20Person%20Character))
  (bind _ingredients (Variables|/Game/ThirdPerson/Blueprints/BP_ThirdPersonCharacter.BP_ThirdPersonCharacter_C|GetIngredients _as_bp_third_person_character))
  (bind _index (Utilities|FlowControl|ForLoopwithBreak 0 (- (Utilities|Array|Length (Variables|/Game/ThirdPerson/Blueprints/BP_ThirdPersonCharacter.BP_ThirdPersonCharacter_C|GetIngredients (Variables|Default|GetAs%20BP%20Third%20Person%20Character))) 1) :!label _label)
    (:LoopBody
      (if (Utilities|Enum|Equal(Enum) (Variables|/Game/Dev/Collectibles/BP_Ingredient.BP_Ingredient_C|GetInstance_name (Utilities|Array|Get(acopy) _ingredients _index)) "NewEnumerator6")
        (Utilities|Array|RemoveItem _ingredients (Utilities|Array|Get(acopy) _ingredients _index))
        (LocalVariables|Setfound true)
        (Utilities|FlowControl|Sequence
          (:then_0
            (goto _label Break))
          (:then_1
            (return (LocalVariables|Getfound))))))
    (:Completed
      (if (LocalVariables|Getfound)
        (LocalVariables|Setfound true)
        (else
          (LocalVariables|Setfound false)))
      (return (LocalVariables|Getfound)))))