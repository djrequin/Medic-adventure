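; BP_Chara_Parent is a parent Blueprint for NPCs that the player can talk to.
; On BeginPlay it sets the "Parler" prompt text and converts the Names enum array into strings in HNames.
; PrintInteractionButton passes that prompt to the given widget for display.
; Interaction disables player input and opens a WB_Dialog_system widget fed with the converted names and the Contents data.
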(event EventBeginPlay
  (Variables|Default|SetEntry_text "Parler")
  (CallFunction|ConvertNames))

(event Collision|EventActorBeginOverlap
  (params (OtherActor :type Actor%20Object%20Reference)))

(event EventTick
  (params (DeltaSeconds :type Float%20%28single-precision%29)))

(event EventPrintInteractionButton
  (params (Widget :type WB%20Interaction%20Button%20Object%20Reference))
  (Default|Print Widget (Variables|Default|GetEntry_text)))

(event EventInteraction
  (Input|DisableInput (Game|GetPlayerCharacter 0) (Game|GetPlayerController 0))
  (bind _returnvalue (UserInterface|CreateWidget "/Game/UI/Story/WB_Dialog_system.WB_Dialog_system_C" 0 (Variables|Default|GetH_Names) (Variables|Default|GetContents)))
  (UserInterface|Viewport|AddtoViewport _returnvalue 0))

(fn ConstructionScript)

(fn ConvertNames
  (for _array_element (Variables|Default|GetNames)
    (Utilities|Array|Add (Variables|Default|GetH_Names) (Utilities|String|EnumtoString _array_element))))