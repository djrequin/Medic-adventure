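; BP_Bracelet is an interactable pickup actor for a bracelet that the player collects.
; Its Interaction event runs once, adding the actor to the RandomObjects array on BP_ThirdPersonCharacter.
; It then shows a WB_Item widget with the item's image, name and possessed flag, and teleports its root component to the world origin instead of destroying itself.
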(event EventBeginPlay
  (|CallParentFunction) ; This node is disabled and will not be called.\nDrag off pins to build functionality.
)

(event Collision|EventActorBeginOverlap
  (params (OtherActor :type Actor%20Object%20Reference))
  (|CallParentFunction OtherActor) ; This node is disabled and will not be called.\nDrag off pins to build functionality.
)

(event EventTick
  (params (DeltaSeconds :type Float%20%28single-precision%29))
  (|CallParentFunction DeltaSeconds) ; This node is disabled and will not be called.\nDrag off pins to build functionality.
)

(event EventInteraction
  (Utilities|FlowControl|DoOnce false
    (:Completed
      (Utilities|Array|Add (Variables|/Game/ThirdPerson/Blueprints/BP_ThirdPersonCharacter.BP_ThirdPersonCharacter_C|GetRandom_objects (.AsBP%20Third%20Person%20Character (Utilities|Casting|CastToBP_ThirdPersonCharacter (Game|GetPlayerCharacter 0)))) self)
      (bind _returnvalue (UserInterface|CreateWidget "/Game/UI/Character/WB_Item.WB_Item_C" 0 (Utilities|Struct|MakeSlateBrush "Image" "NoTile" "NoMirror" "(X=32.000000,Y=32.000000)" "(Left=0.000000,Top=0.000000,Right=0.000000,Bottom=0.000000)" "(SpecifiedColor=(R=1.000000,G=1.000000,B=1.000000,A=1.000000),ColorUseRule=UseColor_Specified)" "(CornerRadii=(X=0.000000,Y=0.000000,Z=0.000000,W=1.000000),Color=(SpecifiedColor=(R=0.000000,G=0.000000,B=0.000000,A=0.000000),ColorUseRule=UseColor_Specified),Width=0.000000,RoundingType=HalfHeightRadius,bUseBrushTransparency=False)" "/Game/Images/sac.sac") (Utilities|Text|ToText(String) (Variables|Default|GetEntry_text)) 1))
      (UserInterface|Viewport|AddtoViewport _returnvalue 0)
      (Transformation|SetWorldLocation (Variables|Default|GetDefaultSceneRoot) "0, 0, 0" false true))))

(fn ConstructionScript
  (|CallParentFunction))